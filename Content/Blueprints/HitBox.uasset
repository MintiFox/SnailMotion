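; HitBox is an actor that deals damage and knockback to IDamageable actors touching it.
; One tick after BeginPlay it hits actors already overlapping its Sphere, and ActorBeginOverlap hits those that overlap it.
; Both paths call OnDamage through the interface, passing Damage, CanDamage and a knockback along the actor's forward vector.
; It destroys itself after LifeTime, unless that is zero.
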(event `self.ReceiveBeginPlay`
  (bind _overlappingactors (`PrimitiveComponent.GetOverlappingActors` (`self.Sphere`) null))
  (`|ExecutionSequence`
    (:`then_0`
      ;[1 1 1] Self Destroy
      (if (not (== (`self.LifeTime`) 0.0))
        (`KismetSystemLibrary.Delay` (`self.LifeTime`))
        (`self.K2_DestroyActor`)))
    (:`then_1`
      (`KismetSystemLibrary.Delay` 0.0)
      (if (> (`KismetArrayLibrary.Array_Length` _overlappingactors) 0)
        ;[1 1 1] Damamge stuff on spawn
        (for _array_element _overlappingactors
          (if (`KismetSystemLibrary.IsValid` _array_element)
            (bind _asidamageable (cast `/Game/Blueprints/Interfaces/IDamageable` _array_element))
            (`/Game/Blueprints/Interfaces/IDamageable.OnDamage` _asidamageable (`self.Damage`) (* (`self.GetActorForwardVector`) (`self.Knockback`)) (`self.Can Damage`))))))))

(event `self.ReceiveActorBeginOverlap`
  (params (OtherActor :type "Actor Object Reference"))
  ;[1 1 1] Damage stuff on overlap
  (if (`KismetSystemLibrary.IsValid` OtherActor)
    (bind _asidamageable (cast `/Game/Blueprints/Interfaces/IDamageable` OtherActor))
    (`/Game/Blueprints/Interfaces/IDamageable.OnDamage` _asidamageable (`self.Damage`) (* (`self.GetActorForwardVector`) (`self.Knockback`)) (`self.Can Damage`))))

(fn `UserConstructionScript`)