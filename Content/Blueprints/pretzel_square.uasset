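; Pretzel square actor that repeatedly rotates around its roll axis.
; On BeginPlay it waits an Offset delay, then starts a self-repeating Rotate event.
; Each cycle plays the Turn timeline, adding its Rot track to the roll captured at the start while keeping pitch and yaw fixed.
; When the timeline finishes, it waits Delay seconds before rotating again.
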(event `self.ReceiveBeginPlay`
  (`KismetSystemLibrary.Delay` (`self.Offset`))
  (`self.Rotate`))

(event `Rotate`
  ;[1 1 1] Rotate
  (set `self.Rotation` (.rotation (`self.GetTransform`)))
  (bind (_direction _rot) (`Timeline|Turn` :!via `PlayFromStart`)
    (:`Update`
      (`self.K2_SetActorRotation` (`KismetMathLibrary.MakeRotator` (+ _rot (.roll (`self.Rotation`))) (.pitch (`self.Rotation`)) (.yaw (`self.Rotation`)))))
    (:`Finished`
      (`KismetSystemLibrary.Delay` (`self.Delay`))
      (`self.Rotate`))))

(fn `UserConstructionScript`)