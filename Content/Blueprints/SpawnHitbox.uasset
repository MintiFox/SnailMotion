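; SpawnHitbox is an animation notify that spawns a hitbox actor when it fires during an animation.
; It places the hitbox by adding an offset to the mesh's relative location and transforming that by the owning actor's transform.
; The notify's variables then set the hitbox's lifetime, damage flag, sphere radius and damage amount, so each animation placement can define its own hit.
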(fn `Received_Notify`
  (params (MeshComp :type "SkeletalMeshComponent Object Reference") (Animation :type "AnimSequenceBase Object Reference") (EventReference :type "AnimNotifyEventReference Structure (by ref)"))
  (returns (ReturnValue :type Boolean))
  (bind _returnvalue (`|SpawnActorFromClass` "/Game/Blueprints/HitBox.HitBox_C" (`KismetMathLibrary.MakeTransform` (`KismetMathLibrary.TransformLocation` (`Actor.GetTransform` (`ActorComponent.GetOwner` MeshComp)) (+ (`SceneComponent.RelativeLocation` MeshComp) (`self.LocationOffset`)))) "Undefined" "OverrideRootScale" null null))
  (set `/Game/Blueprints/HitBox.LifeTime` (`self.LifeTime`) _returnvalue)
  (set `/Game/Blueprints/HitBox.Can Damage` (`self.CanHit`) _returnvalue)
  (`SphereComponent.SetSphereRadius` (`/Game/Blueprints/HitBox.Sphere` _returnvalue) (`self.Radius`) true)
  (set `/Game/Blueprints/HitBox.Damage` (`self.Damage`) _returnvalue)
  (return false))