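; FountainBottle is a fountain hazard whose column rises and falls in an endless loop.
; After a start offset, a timeline drives the column height, with separate speeds and hold times for each direction.
; Overlapping players are launched along the actor's up axis if rolled up in their shell, otherwise damaged.
; While any player stays overlapped, Tick keeps pushing them upward with a velocity-scaled drag term, regardless of shell state.
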(event `self.ReceiveBeginPlay`
  (`KismetSystemLibrary.Delay` (`self.Offset`))
  (set `self.StartPos` (`SceneComponent.RelativeLocation` (`self.Collumn`)))
  (`self.MoveColumn` (`self.Up`)))

(event `MoveColumn`
  (params (Up :type Boolean))
  (bind _up (`self.Up`))
  ;[1 1 1] Go Up
  (if Up
    (`TimelineComponent.SetPlayRate` (`self.FlowUp`) (`self.UpSpeed`))
    (bind (_direction _height) (`Timeline|FlowUp` :!via `PlayFromStart` :!label _label)
      (:`Update`
        (`SceneComponent.K2_SetRelativeLocation` (`self.Collumn`) (`KismetMathLibrary.MakeVector` 0.0 0.0 (+ (* _height (`self.Height`)) (.z (`self.StartPos`)))) false false))
      (:`Finished`
        (if (`self.Up`)
          (`KismetSystemLibrary.Delay` (`self.UpHoldTime`))
          (else
            (`KismetSystemLibrary.Delay` (`self.DownHoldTime`))))
        (set `self.Up` (not _up))
        (`self.MoveColumn` _up)))
    (else
      (`TimelineComponent.SetPlayRate` (`self.FlowUp`) (`self.DownSpeed`))
      (goto _label :!via `ReverseFromEnd`))))

(event `self.ReceiveActorBeginOverlap`
  (params (OtherActor :type "Actor Object Reference"))
  ;[1 1 1] On overlap
  (bind _asbp_player_base (cast `/Game/Blueprints/BP_PlayerBase` OtherActor))
  (bind _output_get (set `self.OverlappedPlayer` _asbp_player_base))
  (if (`/Game/Blueprints/BP_PlayerBase.IsRolledUp` _output_get)
    ;[1 1 1] If in shell, launch player
    (`Character.LaunchCharacter` (`self.OverlappedPlayer`) (* (`KismetMathLibrary.TransformDirection` (`self.GetTransform`) (0.0 0.0 1.0)) (`self.ForceKick`)) true true)
    (else
      ;[1 1 1] If not in shell, damage player
      (`/Game/Blueprints/BP_PlayerBase.Damage` (`self.OverlappedPlayer`) (`self.Damage`))))
  (set `self.PlayerOverlapping` true))

(event `self.ReceiveActorEndOverlap`
  (params (OtherActor :type "Actor Object Reference"))
  ;[1 1 1] set flag on overlap end
  (set `self.PlayerOverlapping` false)
  (set `self.OverlappedPlayer` null))

(event `self.ReceiveTick`
  (params (DeltaSeconds :type "Float (single-precision)"))
  ;[1 1 1] Continue pushing player while in fountain
  (if (and (`self.PlayerOverlapping`) (`KismetSystemLibrary.IsValid` (`self.OverlappedPlayer`)))
    (`Character.LaunchCharacter` (`self.OverlappedPlayer`) (+ (* (`self.GetVelocity` (`self.OverlappedPlayer`)) (`self.DragForce`)) (* (`KismetMathLibrary.TransformDirection` (`self.GetTransform`) (0.0 0.0 1.0)) (`self.ForceSustain`))) false false)))

(fn `UserConstructionScript`)