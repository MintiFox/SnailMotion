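; Base player character with camera-relative walk, sprint, limited jumps and a momentum-driven shell roll, plus a traced drop shadow.
; Tick switches between walking and Rolling, where ground-normal traces and curves adjust speed and steering on slopes.
; Fast head-on wall hits bounce the player back, and low speed unrolls the shell.
; Damage grants brief invincibility and is ignored while rolled; death shows a widget, then reloads the level.
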(event `self.ReceiveTick`
  (params (DeltaSeconds :type "Float (single-precision)"))
  (bind _returnvalue (`self.K2_GetActorLocation`))
  (bind _returnvalue_2 (`self.K2_GetActorLocation`))
  (bind _moveinput (`self.MoveInput`))
  (bind _mesh (`self.Mesh`))
  (bind (_returnvalue_x _returnvalue_y _returnvalue_z) (`KismetMathLibrary.BreakVector` (`SceneComponent.K2_GetComponentLocation` (`self.CapsuleComponent`))))
  (bind _returnvalue_3 (`CurveFloat.GetFloatValue` (`self.GroundSteepnessSpeedModCurve`) (`self.GroundSteepnessSpeedModifier`)))
  (bind _returnvalue_4 (`KismetMathLibrary.FClamp` (* (`self.RollAnimSpeed`) (`self.RollVelocity`)) 0.0 50.0))
  (bind _returnvalue_5 (`KismetMathLibrary.Conv_VectorToRotator` (`SceneComponent.GetForwardVector` (`self.CapsuleComponent`))))
  (bind _returnvalue_6 (`KismetMathLibrary.RInterpTo_Constant` _returnvalue_5 (select `bool` (> (`KismetMathLibrary.VSizeSquared` _moveinput) 0.0) :`false` _returnvalue_5 :`true` (`KismetMathLibrary.Conv_VectorToRotator` (`KismetMathLibrary.Normal` _moveinput))) (`GameplayStatics.GetWorldDeltaSeconds`) (`self.RollTurnSpeed`)))
  (if (not (`NavMovementComponent.IsFalling` (`self.CharacterMovement`)))
    (set `self.LastGroundedHeight` _returnvalue_z))
  (`self.UpdateDropShadow`)
  (if (`self.IsRolledUp`)
    (if (< (`KismetMathLibrary.DegAcos` (`KismetMathLibrary.Dot_VectorVector` (`KismetMathLibrary.Normal` (`SceneComponent.GetForwardVector` (`self.CapsuleComponent`))) (`KismetMathLibrary.Normal` (`self.MoveInput`)))) 165.0)
      (bind _output (`self.MoveTowards` (`self.RollVelocity`) (+ (* (`self.RollVelocityTarget`) (`KismetMathLibrary.VSizeXY` (`KismetMathLibrary.Normal` (`self.MoveInput`)))) (* _returnvalue_3 -20.0)) (+ (`self.RolVelocityAcceleration`) (`KismetMathLibrary.Abs` _returnvalue_3))))
      (bind _output_get (set `self.RollVelocity` _output))
      (set `CharacterMovementComponent.MaxWalkSpeed` _output_get (`self.CharacterMovement`))
      (bind _outhit (`KismetSystemLibrary.LineTraceSingle` _returnvalue (+ _returnvalue (0.0 0.0 -200.0)) "TraceTypeQuery1"))
      (set `self.GroundSteepnessSpeedModifier` (`KismetMathLibrary.DegAcos` (`KismetMathLibrary.Dot_VectorVector` (`.Normal` (`GameplayStatics.BreakHitResult` _outhit)) (`KismetMathLibrary.Conv_RotatorToVector` _returnvalue_6))))
      (else
        (bind _output_2 (`self.MoveTowards` (`self.RollVelocity`) 0.0 (`self.RolVelocityAcceleration`)))
        (bind _output_get_2 (set `self.RollVelocity` (* _output_2 (`self.RollStopSpeed`))))
        (set `CharacterMovementComponent.MaxWalkSpeed` _output_get_2 (`self.CharacterMovement`))
        (`self.AddMovementInput` (`SceneComponent.GetForwardVector` (`self.CapsuleComponent`)))))
    (bind (_x _y) (`KismetMathLibrary.BreakVector3f` (`.Normal` (`GameplayStatics.BreakHitResult` _outhit))))
    (`self.AddMovementInput` (`KismetMathLibrary.Conv_RotatorToVector` (`KismetMathLibrary.RInterpTo_Constant` _returnvalue_6 (select `bool` (and (!= (`.Normal` (`GameplayStatics.BreakHitResult` _outhit)) (0.0 0.0 1.0) :`ErrorTolerance` 0.1) (!= (`.Normal` (`GameplayStatics.BreakHitResult` _outhit)) (0.0 0.0 0.0) :`ErrorTolerance` 0.1)) :`false` _returnvalue_6 :`true` (`KismetMathLibrary.Conv_VectorToRotator` (`KismetMathLibrary.Normal` (`KismetMathLibrary.MakeVector` _x _y)))) (`GameplayStatics.GetWorldDeltaSeconds`) (`CurveFloat.GetFloatValue` (`self.GroundSteepnessCurve`) (`KismetMathLibrary.DegAcos` (`KismetMathLibrary.Dot_VectorVector` (`.Normal` (`GameplayStatics.BreakHitResult` _outhit)) (0.0 0.0 1.0)))))))
    (bind _outhit_2 (`KismetSystemLibrary.LineTraceSingle` _returnvalue_2 (+ _returnvalue_2 (* (`SceneComponent.GetForwardVector` (`self.CapsuleComponent`)) (`self.BonkCheckDistance`))) "TraceTypeQuery1"))
    (if (< (`KismetMathLibrary.Dot_VectorVector` (`.Normal` (`GameplayStatics.BreakHitResult` _outhit_2)) (`SceneComponent.GetForwardVector` (`self.CapsuleComponent`))) -0.8)
      (if (> (`self.RollVelocity`) 1000.0)
        (`self.LaunchCharacter` (+ (* (`SceneComponent.GetForwardVector` (`self.CapsuleComponent`)) -1.0 700.0) (`KismetMathLibrary.MakeVector` 0.0 0.0 500.0)) true true)
        (set `self.RollVelocity` 0.0)))
    (`SceneComponent.K2_AddRelativeRotation` _mesh (`KismetMathLibrary.MakeRotator` _returnvalue_4) false false)
    (`SceneComponent.K2_AddLocalOffset` _mesh (+ (`KismetMathLibrary.MakeVector` 0.0 (* _returnvalue_4 -1.0)) (* (`KismetMathLibrary.GetForwardVector` (`KismetMathLibrary.MakeRotator` _returnvalue_4)) (`self.RollCenterDistance`))) false true)
    (set `self.MoveInput` (0.0 0.0 0.0))
    (if (> (`self.MinRollSpeed`) (`self.RollVelocity`))
      (`KismetSystemLibrary.Delay` 0.2)
      (if (and (> (`self.MinRollSpeed`) (`self.RollVelocity`)) (`self.CanJump`))
        (`self.UnRoll`)))
    (else
      ;[1 1 1] Walking
      (`self.AddMovementInput` (`self.MoveInput`))
      (set `self.MoveInput` (0.0 0.0 0.0)))))

(event `self.ReceiveBeginPlay`
  ;[1 1 1] variable initializing
  (set `self.DefaultWalkSpeed` (`CharacterMovementComponent.MaxWalkSpeed` (`self.CharacterMovement`)))
  (set `self.DefaultGravity` (`CharacterMovementComponent.GravityScale` (`self.CharacterMovement`)))
  (set `self.CamManager` (`GameplayStatics.GetPlayerCameraManager` 0)))

(event `Damage`
  (params (Damage :type Integer))
  ;[1 1 1] Damage
  (if (not (or (`self.IsInvincible`) (`self.IsRolledUp`)))
    (if (> Damage (+ (`self.Health`) -1))
      (if (== (`self.Health`) 1)
        (`self.Kill`)
        (set `self.Health` 0)
        (else
          (set `self.Health` 1)))
      (else
        (set `self.Health` (- (`self.Health`) Damage))))
    (set `self.IsInvincible` true)
    (`KismetSystemLibrary.Delay` (`self.InvincibilityTime`))
    (set `self.IsInvincible` false)
    (`KismetSystemLibrary.PrintString` (`KismetStringLibrary.Concat_StrStr` "Took " (`KismetStringLibrary.Conv_IntToString` Damage) " damage." (`KismetStringLibrary.Conv_IntToString` (`self.Health`)) " health left."))))

(event `/Game/Blueprints/Interfaces/IDamageable.OnDamage`
  (params (Damage :type Integer) (Knockback :type "Vector Structure") (DamageSource :type "/Game/Assets/DamageSource Enum" :default "NewEnumerator0"))
  (`self.Damage` Damage))

(event `Kill`
  ;[1 1 1] Death
  (if (not (`self.IsRolledUp`))
    (`PrimitiveComponent.SetSimulatePhysics` (`self.Mesh`) true))
  (bind _returnvalue (`|CreateWidget` "/Game/Assets/Widgets/Death.Death_C"))
  (`UserWidget.AddToViewport` _returnvalue 0)
  (`self.DisableInput` (`GameplayStatics.GetPlayerController` 0))
  (`SceneComponent.K2_DetachFromComponent` (`self.SpringArm`) "KeepWorld" "KeepWorld" "KeepWorld" true)
  (`KismetSystemLibrary.Delay` 2.5)
  (bind _returnvalue_2 (`GameplayStatics.GetCurrentLevelName` true))
  (`KismetSystemLibrary.ExecuteConsoleCommand` (`KismetStringLibrary.Concat_StrStr` "open " _returnvalue_2) null))

(event `Key|Z`
  (params (Key :type "Key Structure"))
  (:`Pressed`
    (`self.Kill`)))

(event `InputAxis|MoveForward`
  (params (AxisValue :type "Float (single-precision)"))
  ;[1 1 1] Movement
  (set `self.MoveInput` (+ (* (`KismetMathLibrary.GetForwardVector` (`KismetMathLibrary.MakeRotator` 0.0 0.0 (.yaw (`PlayerCameraManager.GetCameraRotation` (`self.CamManager`))))) AxisValue) (`self.MoveInput`))))

(event `InputAxis|Turn`
  (params (AxisValue :type "Float (single-precision)"))
  ;[1 1 1] Cam Look
  (`self.AddControllerYawInput` AxisValue))

(event `InputAction|Sprint`
  (params (Key :type "Key Structure"))
  ;[1 1 1] Sprint/Walk
  (:`Pressed`
    (set `CharacterMovementComponent.MaxWalkSpeed` (* (`self.DefaultWalkSpeed`) (`self.SprintMultiplier`)) (`self.CharacterMovement`)))
  (:`Released`
    (set `CharacterMovementComponent.MaxWalkSpeed` (`self.DefaultWalkSpeed`) (`self.CharacterMovement`))))

(event `InputAxis|MoveRight`
  (params (AxisValue :type "Float (single-precision)"))
  ;[1 1 1] Movement
  (set `self.MoveInput` (+ (* AxisValue (`KismetMathLibrary.GetRightVector` (`KismetMathLibrary.MakeRotator` 0.0 0.0 (.yaw (`PlayerCameraManager.GetCameraRotation` (`self.CamManager`)))))) (`self.MoveInput`))))

(event `InputAxis|LookUp`
  (params (AxisValue :type "Float (single-precision)"))
  ;[1 1 1] Cam Look
  (`self.AddControllerPitchInput` AxisValue))

(event `InputAction|Jump`
  (params (Key :type "Key Structure"))
  ;[1 1 1] Jumping
  (:`Pressed`
    (`self.Try Jump`))
  (:`Released`
    (`self.StopJumping`)))

(event `self.OnLanded`
  (params (Hit :type "HitResult Structure (by ref)"))
  ;[1 1 1] On Landed
  (set `self.JumpCount` 0))

(event `InputAction|Roll`
  (params (Key :type "Key Structure"))
  ;[1 1 1] On Roll / Unroll
  (:`Pressed`
    (if (not (`self.IsRolledUp`))
      (`self.Roll`)
      (`self.LaunchCharacter` (+ (`KismetMathLibrary.MakeVector` 0.0 0.0 (`self.RollUpwardKick`)) (* (`SceneComponent.GetForwardVector` (`self.CapsuleComponent`)) (`self.RollForwardKick`))) true true))))

(event `Roll`
  ;[1 1 1] On Roll / Unroll
  (set `self.IsRolledUp` true)
  (set `self.RollVelocity` (`self.RollStartVelocity`))
  (`CapsuleComponent.SetCapsuleHalfHeight` (`self.CapsuleComponent`) 40.0 true)
  (`SceneComponent.K2_SetRelativeLocation` (`self.Mesh`) (0.0 0.0 -40.0) false true))

(event `UnRoll`
  (bind _mesh (`self.Mesh`))
  ;[1 1 1] On Roll / Unroll
  (set `self.IsRolledUp` false)
  (set `self.IsInvincible` true)
  (set `CharacterMovementComponent.MaxWalkSpeed` (`self.DefaultWalkSpeed`) (`self.CharacterMovement`))
  (`SceneComponent.ResetRelativeTransform` (`self.Mesh`))
  (`SceneComponent.K2_SetRelativeLocation` _mesh (0.0 0.0 -90.0) false true)
  (`SceneComponent.K2_SetRelativeRotation` _mesh (struct :`Yaw` -90.0) false false)
  (`SceneComponent.SetRelativeScale3D` _mesh (20.0 20.0 20.0))
  (`CapsuleComponent.SetCapsuleHalfHeight` (`self.CapsuleComponent`) 88.0 true)
  (`self.K2_AddActorWorldOffset` (0.0 0.0 48.0))
  (`KismetSystemLibrary.Delay` 0.2)
  (set `self.IsInvincible` false))

(fn `MoveTowards`
  (params (Value :type "Float (double-precision)") (Target :type "Float (double-precision)") (MaxInterp :type "Float (double-precision)"))
  (returns (Output :type "Float (double-precision)"))
  (bind _returnvalue (+ Value MaxInterp))
  (bind _returnvalue_2 (- Value (`self.RollVelocityDeceleration`)))
  (if (> Value Target)
    (if (> _returnvalue_2 Target)
      (return _returnvalue_2)
      (else
        (return Target)))
    (elif (> _returnvalue Target)
      (return Target)
      (else
        (return _returnvalue)))))

(fn `ResetJumpVelocity`
  (bind (_returnvalue_x _returnvalue_y) (`KismetMathLibrary.BreakVector` (`self.GetVelocity`)))
  (set `MovementComponent.Velocity` (`KismetMathLibrary.MakeVector` _returnvalue_x _returnvalue_y) (`self.CharacterMovement`)))

(fn `Try Jump`
  (if (< (`self.JumpCount`) (`self.JumpMaxCount`))
    (if (not (`NavMovementComponent.IsFalling` (`self.CharacterMovement`)))
      (if (not (`self.IsRolledUp`))
        (`self.PlayAnimMontage` "/Game/Assets/Meshes/Drizzle/Drizzle_Anim_Jump.Drizzle_Anim_Jump"))
      ;[1 1 1] Ground Jump
      (`self.ResetJumpVelocity`)
      (`self.Jump`)
      (`/Engine/EditorBlueprintResources/StandardMacros.IncrementInt` (`self.JumpCount`)))))

(fn `UpdateDropShadow`
  (bind _returnvalue (`SceneComponent.K2_GetComponentLocation` (`self.CapsuleComponent`)))
  (bind _outhit (`KismetSystemLibrary.LineTraceSingle` _returnvalue (+ _returnvalue (0.0 0.0 -2000.0)) "TraceTypeQuery1"))
  (`SceneComponent.K2_SetWorldLocation` (`self.DropShadow`) (`.Location` (`GameplayStatics.BreakHitResult` _outhit)) false true))

(fn `UserConstructionScript`)