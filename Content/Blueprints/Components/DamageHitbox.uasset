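; DamageHitbox is a component that damages actors overlapping its owning actor.
; On BeginPlay it binds the owner's overlap events, tracking overlapping actors in a collection.
; Each new overlap sends damage, knockback and source to actors implementing IDamageable through OnDamageMessage.
; An unconnected, experimental loop for repeatedly hitting lingering actors through Hit never runs, so damage applies only on entry.
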(event `OnActorEndOverlap_Event_0`
  (params (OverlappedActor :type "Actor Object Reference") (OtherActor :type "Actor Object Reference"))
  (`BlueprintSetLibrary.Set_Remove` (`self.Overlapping Actors`) OtherActor))

(event `self.ReceiveBeginPlay`
  (add `Actor.OnActorBeginOverlap` (`self.GetOwner`) (delegate `OnActorBeginOverlap_Event_0`))
  (add `Actor.OnActorEndOverlap` (`self.GetOwner`) (delegate `OnActorEndOverlap_Event_0`)))

(event `OnActorBeginOverlap_Event_0`
  (params (OverlappedActor :type "Actor Object Reference") (OtherActor :type "Actor Object Reference"))
  (`BlueprintSetLibrary.Set_Add` (`self.Overlapping Actors`) OtherActor)
  (if (`KismetSystemLibrary.DoesImplementInterface` OtherActor "/Game/Blueprints/Interfaces/IDamageable.IDamageable_C")
    (message `/Game/Blueprints/Interfaces/IDamageable.OnDamage` OtherActor (`self.Damage`) (`self.Knockback`) (`self.Damage Source`))))

(fn `hit`
  (params (ActorToHit :type "Actor Object Reference"))
  (if (`KismetSystemLibrary.DoesImplementInterface` ActorToHit "/Game/Blueprints/Interfaces/IDamageable.IDamageable_C")
    (message `/Game/Blueprints/Interfaces/IDamageable.OnDamage` ActorToHit (`self.Damage`) (`self.Knockback`) (`self.Damage Source`))))