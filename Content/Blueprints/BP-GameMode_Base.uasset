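; Base game mode that sets up the level camera and the player's costume when play begins.
; BeginPlay spawns a PlayerLevelCamera at the game mode's transform and caches it, then caches the first player pawn as BP_PlayerBase.
; The costume is applied by copying the FoodDye materials onto the player's mesh, matching array index to material slot.
; Tick and the construction script are empty.
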(event `self.ReceiveBeginPlay`
  (bind _returnvalue (`|SpawnActorFromClass` "/Game/Blueprints/Camera/PlayerLevelCamera.PlayerLevelCamera_C" (`self.GetTransform`) "Undefined" "OverrideRootScale" null null))
  (set `self.Cam` _returnvalue)
  (bind _asbp_player_base (cast `/Game/Blueprints/BP_PlayerBase` (`GameplayStatics.GetPlayerPawn` 0)))
  (set `self.Player` _asbp_player_base)
  ;[1 1 1] Set costume
  (for (_array_element _array_index) (`/Game/Assets/CostumeMaterials/CostumeMaterialSet.Materials` (`self.FoodDye`))
    (`PrimitiveComponent.SetMaterial` (`Character.Mesh` (`self.Player`)) _array_index _array_element)))

(fn `UserConstructionScript`)