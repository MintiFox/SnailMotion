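; Camera door trigger that switches the game mode's shared camera between CamA and CamB as the player passes through.
; Two half-overlapping boxes, sized and labelled in the construction script, infer direction from which one the player exits while still inside the other.
; A zero TransitionSpeed jump-cuts; otherwise a curve-driven timeline blends at that play rate, reverses for the opposite direction, and settles on the end camera.
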(event `self.ReceiveBeginPlay`
  (`KismetSystemLibrary.Delay` 0.0)
  (bind _asbp_game_mode_base (cast `/Game/Blueprints/BP-GameMode_Base` (`GameplayStatics.GetGameMode`)))
  (set `self.Cam` (`/Game/Blueprints/BP-GameMode_Base.Cam` _asbp_game_mode_base)))

(event `self.A.OnComponentBeginOverlap`
  (params (OverlappedComponent :type "PrimitiveComponent Object Reference") (OtherActor :type "Actor Object Reference") (OtherComp :type "PrimitiveComponent Object Reference") (OtherBodyIndex :type Integer) (bFromSweep :type Boolean) (SweepResult :type "HitResult Structure (by ref)"))
  (cast `/Game/Blueprints/BP_PlayerBase` OtherActor)
  (set `self.AOverlap` true))

(event `self.A.OnComponentEndOverlap`
  (params (OverlappedComponent :type "PrimitiveComponent Object Reference") (OtherActor :type "Actor Object Reference") (OtherComp :type "PrimitiveComponent Object Reference") (OtherBodyIndex :type Integer))
  (cast `/Game/Blueprints/BP_PlayerBase` OtherActor)
  (set `self.AOverlap` false)
  ;[1 1 1] Going from B to A
  (if (`self.BOverlap`)
    (if (== (`self.TransitionSpeed`) 0.0)
      (set `/Game/Blueprints/Camera/PlayerLevelCamera.CurrentTarget` (`self.CamB`) (`self.Cam`))
      (set `/Game/Blueprints/Camera/PlayerLevelCamera.BlendTarget` null (`self.Cam`))
      (`KismetSystemLibrary.Delay` 0.0)
      (`/Game/Blueprints/Camera/PlayerLevelCamera.JumpCut` (`self.Cam`))
      (else
        (`TimelineComponent.SetPlayRate` (`self.CamTransitionTimeline`) (`self.TransitionSpeed`))
        (`|ExecutionSequence`
          (:`then_0`
            (set `/Game/Blueprints/Camera/PlayerLevelCamera.CurrentTarget` (`self.CamA`) (`self.Cam`) :!label _label)
            (set `/Game/Blueprints/Camera/PlayerLevelCamera.BlendTarget` (`self.CamB`) (`self.Cam`)))
          (:`then_1`
            (if (`TimelineComponent.IsPlaying` (`self.CamTransitionTimeline`))
              (bind (_direction _t) (`Timeline|CamTransitionTimeline` :!label _label_2)
                (:`Update`
                  (set `/Game/Blueprints/Camera/PlayerLevelCamera.BlendPercent` (`CurveFloat.GetFloatValue` (`self.CamTransitionCurve`) _t) (`self.Cam`)))
                (:`Finished`
                  (set `/Game/Blueprints/Camera/PlayerLevelCamera.CurrentTarget` (select `bool` (> _t 0.5) :`false` (`self.CamA`) :`true` (`self.CamB`)) (`self.Cam`))
                  (set `/Game/Blueprints/Camera/PlayerLevelCamera.BlendTarget` null (`self.Cam`))))
              (else
                (goto _label_2 :!via `PlayFromStart`)))))))))

(event `self.B.OnComponentBeginOverlap`
  (params (OverlappedComponent :type "PrimitiveComponent Object Reference") (OtherActor :type "Actor Object Reference") (OtherComp :type "PrimitiveComponent Object Reference") (OtherBodyIndex :type Integer) (bFromSweep :type Boolean) (SweepResult :type "HitResult Structure (by ref)"))
  (cast `/Game/Blueprints/BP_PlayerBase` OtherActor)
  (set `self.BOverlap` true))

(event `self.B.OnComponentEndOverlap`
  (params (OverlappedComponent :type "PrimitiveComponent Object Reference") (OtherActor :type "Actor Object Reference") (OtherComp :type "PrimitiveComponent Object Reference") (OtherBodyIndex :type Integer))
  (cast `/Game/Blueprints/BP_PlayerBase` OtherActor)
  (set `self.BOverlap` false)
  ;[1 1 1] Going from A to B
  (if (`self.AOverlap`)
    (if (== (`self.TransitionSpeed`) 0.0)
      (set `/Game/Blueprints/Camera/PlayerLevelCamera.CurrentTarget` (`self.CamA`) (`self.Cam`))
      (set `/Game/Blueprints/Camera/PlayerLevelCamera.BlendTarget` null (`self.Cam`))
      (`KismetSystemLibrary.Delay` 0.0)
      (`/Game/Blueprints/Camera/PlayerLevelCamera.JumpCut` (`self.Cam`))
      (else
        (`TimelineComponent.SetPlayRate` (`self.CamTransitionTimeline`) (`self.TransitionSpeed`))
        (`|ExecutionSequence`
          (:`then_0`
            (goto _label))
          (:`then_1`
            (if (`TimelineComponent.IsPlaying` (`self.CamTransitionTimeline`))
              (goto _label_2 :!via `Reverse`)
              (else
                (goto _label_2 :!via `ReverseFromEnd`)))))))))

(fn `UserConstructionScript`
  (bind _boxsize_x (`KismetMathLibrary.BreakVector` (`self.BoxSize`)))
  (bind (_boxsize_x_2 _boxsize_y _boxsize_z) (`KismetMathLibrary.BreakVector` (`self.BoxSize`)))
  (bind (_boxsize_x_3 _boxsize_y_2) (`KismetMathLibrary.BreakVector` (`self.BoxSize`)))
  (bind (_boxsize_x_4 _boxsize_y_3) (`KismetMathLibrary.BreakVector` (`self.BoxSize`)))
  (bind (_returnvalue_x _returnvalue_y _returnvalue_z) (`KismetMathLibrary.BreakVector` (* (`BoxComponent.GetScaledBoxExtent` (`self.A`)) 1.0)))
  (bind (_returnvalue_x_2 _returnvalue_y_2 _returnvalue_z_2) (`KismetMathLibrary.BreakVector` (* (`BoxComponent.GetScaledBoxExtent` (`self.A`)) 1.0)))
  (`BoxComponent.SetBoxExtent` (`self.A`) (* (`self.BoxSize`) 0.5) true)
  (`SceneComponent.K2_SetRelativeLocation` (`self.A`) (* (`self.BoxSize`) 0.5) false false)
  (`BoxComponent.SetBoxExtent` (`self.B`) (* (`self.BoxSize`) 0.5) true)
  (`SceneComponent.K2_SetRelativeLocation` (`self.B`) (+ (* (`self.BoxSize`) 0.5) (`KismetMathLibrary.MakeVector` (* _boxsize_x 0.5))) false false)
  (`SceneComponent.K2_AddLocalOffset` (`self.AText`) (`KismetMathLibrary.MakeVector` 0.0 _returnvalue_y_2 _returnvalue_z_2) false false)
  (`SceneComponent.K2_AddLocalOffset` (`self.BText`) (`KismetMathLibrary.MakeVector` (* _returnvalue_x 2.0) _returnvalue_y _returnvalue_z) false false)
  (`TextRenderComponent.SetWorldSize` (`self.AText`) (`KismetMathLibrary.FClamp` (* _boxsize_y_3 0.5) 0.0 500.0))
  (`TextRenderComponent.SetWorldSize` (`self.BText`) (`KismetMathLibrary.FClamp` (* _boxsize_y_2 0.5) 0.0 500.0))
  (set `self.BoxSize` (`KismetMathLibrary.MakeVector` 20.0 _boxsize_y _boxsize_z)))