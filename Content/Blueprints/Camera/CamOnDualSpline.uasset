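; Camera rig that follows the player along two nested splines, using a CameraActor spawned at the offset actor's transform on BeginPlay.
; Each tick, Spline2 eases toward the point on Spline nearest the player pawn plus Offset, and the camera eases toward the nearest point on Spline2 plus the same Offset.
; Smoothing is a fixed-alpha lerp per frame, and the graph never updates camera rotation or sets the view target.
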(event `self.ReceiveBeginPlay`
  (`parent.ReceiveBeginPlay`)
  (bind _returnvalue (`|SpawnActorFromClass` "/Script/Engine.CameraActor" (`SceneComponent.K2_GetComponentToWorld` (`self.OfssetActor`)) "Undefined" "OverrideRootScale" null null))
  (set `self.Cam` _returnvalue))

(event `self.ReceiveTick`
  (params (DeltaSeconds :type "Float (single-precision)"))
  (bind _returnvalue_location (`KismetMathLibrary.BreakTransform` (`self.GetTransform` (`GameplayStatics.GetPlayerPawn` 0))))
  (bind _returnvalue_location_2 (`KismetMathLibrary.BreakTransform` (`self.GetTransform` (`GameplayStatics.GetPlayerPawn` 0))))
  (`SceneComponent.K2_SetWorldLocation` (`self.Spline2`) (`KismetMathLibrary.VLerp` (`SceneComponent.K2_GetComponentLocation` (`self.Spline2`)) (+ (`SplineComponent.FindLocationClosestToWorldLocation` (`self.Spline`) _returnvalue_location_2 "World") (`self.Offset`)) 0.1) false false)
  (`self.K2_SetActorLocation` (`self.Cam`) (`KismetMathLibrary.VLerp` (`SceneComponent.K2_GetComponentLocation` (`Actor.RootComponent` (`self.Cam`))) (+ (`SplineComponent.FindLocationClosestToWorldLocation` (`self.Spline2`) _returnvalue_location "World") (`self.Offset`)) 0.1) false false))

(fn `UserConstructionScript`
  (`parent.UserConstructionScript`))