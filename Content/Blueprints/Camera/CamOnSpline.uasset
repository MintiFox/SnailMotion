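; Actor that moves a camera along a spline to follow the player pawn, acting as a rail camera.
; On BeginPlay it stores the offset between a reference actor and its own location.
; Each tick it finds the spline point closest to the player pawn and teleports the camera there plus that offset.
; An unconnected check that would disable ticking when the camera is invalid never runs.
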(event `self.ReceiveBeginPlay`
  (set `self.Offset` (- (`SceneComponent.K2_GetComponentLocation` (`self.OfssetActor`)) (`self.K2_GetActorLocation`))))

(event `self.ReceiveTick`
  (params (DeltaSeconds :type "Float (single-precision)"))
  (bind _returnvalue_location (`KismetMathLibrary.BreakTransform` (`self.GetTransform` (`GameplayStatics.GetPlayerPawn` 0))))
  (`self.K2_SetActorLocation` (`self.Cam`) (+ (`SplineComponent.FindLocationClosestToWorldLocation` (`self.Spline`) _returnvalue_location "World") (`self.Offset`)) false true))

(fn `UserConstructionScript`)