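; Trigger zone that switches the player's view between two cameras as actors enter and leave it.
; Begin overlap blends to view target A and end overlap blends to view target B, each with its own transition time.
; PlayerCamera targets handle their own activation and the opposite one is disabled; other actors use a cubic SetViewTargetWithBlend on player controller 0.
; The overlapping actor is not filtered.
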(event `self.ReceiveActorBeginOverlap`
  (params (OtherActor :type "Actor Object Reference"))
  (bind _asplayer_camera (cast `/Game/Blueprints/Camera/PlayerCamera` (`self.View Target A`))
    (:`then`
      (`/Game/Blueprints/Camera/PlayerCamera.EnableCam` _asplayer_camera (`self.TransitionTimeA`)))
    (:`CastFailed`
      (`PlayerController.SetViewTargetWithBlend` (`GameplayStatics.GetPlayerController` 0) (`self.View Target A`) (`self.TransitionTimeA`) "VTBlend_Cubic" 1.0 false)))
  (bind _asplayer_camera_2 (cast `/Game/Blueprints/Camera/PlayerCamera` (`self.View Target B`)))
  (`/Game/Blueprints/Camera/PlayerCamera.DisableCam` _asplayer_camera_2))

(event `self.ReceiveActorEndOverlap`
  (params (OtherActor :type "Actor Object Reference"))
  (bind _asplayer_camera (cast `/Game/Blueprints/Camera/PlayerCamera` (`self.View Target B`))
    (:`then`
      (`/Game/Blueprints/Camera/PlayerCamera.EnableCam` _asplayer_camera (`self.TransitionTimeB`)))
    (:`CastFailed`
      (`PlayerController.SetViewTargetWithBlend` (`GameplayStatics.GetPlayerController` 0) (`self.View Target B`) (`self.TransitionTimeB`) "VTBlend_Cubic" 1.0 false)))
  (bind _asplayer_camera_2 (cast `/Game/Blueprints/Camera/PlayerCamera` (`self.View Target A`)))
  (`/Game/Blueprints/Camera/PlayerCamera.DisableCam` _asplayer_camera_2))

(fn `UserConstructionScript`)