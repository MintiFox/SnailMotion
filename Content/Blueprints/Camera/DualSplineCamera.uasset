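; Camera actor that follows the player on two nested splines, taking over the view with a blend through EnableCam.
; Each tick the Range spline moves to the Path point nearest the offset player position, then the camera eases toward the nearest point on Range.
; Camera height can track the player's last grounded height, and rotations can follow both curves from their starting deltas.
; AutoSetOffset derives the target offset from a forward line trace.
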(event `self.ReceiveBeginPlay`
  (set `self.StartingCamRotation` (`KismetMathLibrary.NormalizedDeltaRotator` (`SceneComponent.K2_GetComponentRotation` (`self.CameraComponent`)) (`SplineComponent.GetRotationAtTime` (`self.Range`) 0.0 "World" false)))
  (set `self.StartingRangeRotation` (`KismetMathLibrary.NormalizedDeltaRotator` (`SceneComponent.K2_GetComponentRotation` (`self.Range`)) (`SplineComponent.GetRotationAtTime` (`self.Path`) 0.0 "World" false)))
  (set `self.OffsetLocal` (`KismetMathLibrary.InverseTransformLocation` (`SceneComponent.GetRelativeTransform` (`self.CameraComponent`)) (`self.TargetOffset`))))

(event `self.ReceiveTick`
  (params (DeltaSeconds :type "Float (single-precision)"))
  (bind (_targetoffset_x _targetoffset_y _targetoffset_z) (`KismetMathLibrary.BreakVector` (`self.TargetOffset`)))
  (bind _returnvalue (`SceneComponent.K2_GetComponentLocation` (`self.CameraComponent`)))
  (bind _returnvalue_location (`KismetMathLibrary.BreakTransform` (`self.GetTransform` (`GameplayStatics.GetPlayerPawn` 0))))
  (bind _returnvalue_location_2 (`KismetMathLibrary.BreakTransform` (`self.GetTransform` (`GameplayStatics.GetPlayerPawn` 0))))
  (bind _returnvalue_2 (+ _returnvalue_location_2 (`self.TargetOffset`)))
  (bind _returnvalue_3 (+ _returnvalue_location (`self.TargetOffset`)))
  (bind _returnvalue_4 (`SplineComponent.FindLocationClosestToWorldLocation` (`self.Range`) _returnvalue_2 "World"))
  (bind (_x _y) (`KismetMathLibrary.BreakVector3f` _returnvalue_4))
  (bind _output_get (set `self.TargetOffset` (`KismetMathLibrary.TransformDirection` (`SceneComponent.GetRelativeTransform` (`self.CameraComponent`)) (`self.OffsetLocal`))))
  (if (`self.TrackPlayerHeight`)
    (bind _asbp_player_base (cast `/Game/Blueprints/BP_PlayerBase` (`GameplayStatics.GetPlayerPawn` 0))
      (:`then`
        (set `self.PlayerGroundHeight` (`/Game/Blueprints/BP_PlayerBase.LastGroundedHeight` _asbp_player_base)))
      (:`CastFailed`
        _)))
  ;[1 1 1] Move Range along Path
  (`SceneComponent.K2_SetWorldLocation` (`self.Range`) (`SplineComponent.FindLocationClosestToWorldLocation` (`self.Path`) _returnvalue_3 "World") false false)
  (bind _output_get_2 (set `self.TargetLocation` (select `bool` (`self.TrackPlayerHeight`) :`false` _returnvalue_4 :`true` (`KismetMathLibrary.MakeVector` _x _y (+ _targetoffset_z (`self.PlayerGroundHeight`))))))
  (bind (_x_2 _y_2) (`KismetMathLibrary.BreakVector3f` (`KismetMathLibrary.VInterpTo` _returnvalue _output_get_2 DeltaSeconds 5.0)))
  (`SceneComponent.K2_SetWorldLocation` (`self.CameraComponent`) (`KismetMathLibrary.MakeVector` _x_2 _y_2 (`KismetMathLibrary.FInterpTo` (`.Z` (`KismetMathLibrary.BreakVector3f` _returnvalue)) (`.Z` (`KismetMathLibrary.BreakVector3f` _output_get_2)) DeltaSeconds 2.0)) false false)
  (if (`self.FollowCurveRotation`)
    (`SceneComponent.K2_SetWorldRotation` (`self.Range`) (`KismetMathLibrary.RInterpTo` (`SceneComponent.K2_GetComponentRotation` (`self.Range`)) (`KismetMathLibrary.ComposeRotators` (`self.StartingRangeRotation`) (`SplineComponent.FindRotationClosestToWorldLocation` (`self.Path`) _returnvalue_3 "World")) DeltaSeconds 5.0) false false)
    (`SceneComponent.K2_SetWorldRotation` (`self.CameraComponent`) (`KismetMathLibrary.RInterpTo` (`SceneComponent.K2_GetComponentRotation` (`self.CameraComponent`)) (`KismetMathLibrary.ComposeRotators` (`self.StartingCamRotation`) (`SplineComponent.FindRotationClosestToWorldLocation` (`self.Range`) _returnvalue_2 "World")) DeltaSeconds 1.0) false false)))

(event `/Game/Blueprints/Camera/PlayerCamera.EnableCam`
  (params (TransitionTime :type "Float (double-precision)"))
  ;[1 1 1] Enable/Disable Cam
  (`PlayerController.SetViewTargetWithBlend` (`GameplayStatics.GetPlayerController` 0) self TransitionTime "VTBlend_Cubic" 1.0 true)
  (`self.SetActorTickEnabled` true))

(event `/Game/Blueprints/Camera/PlayerCamera.DisableCam`
  ;[1 1 1] Enable/Disable Cam
  (`self.SetActorTickEnabled` false))

(fn `Auto Set Offset`
  (bind _returnvalue (`SceneComponent.K2_GetComponentLocation` (`self.CameraComponent`)))
  (bind _returnvalue_2 (`SceneComponent.K2_GetComponentLocation` (`self.CameraComponent`)))
  (bind _outhit (`KismetSystemLibrary.LineTraceSingle` _returnvalue_2 (+ _returnvalue_2 (* (`SceneComponent.GetForwardVector` (`self.CameraComponent`)) 5000.0)) "TraceTypeQuery1"))
  (bind _output_get (set `self.TargetOffset` (- _returnvalue (`.Location` (`GameplayStatics.BreakHitResult` _outhit)))))
  (`KismetSystemLibrary.DrawDebugSphere` (* (- _output_get _returnvalue) -1.0) 100.0 12 (struct :`R` 1.0 :`G` 1.0 :`B` 1.0 :`A` 1.0) 1.0))

(fn `RotateAround`
  (params (Center :type "Vector Structure") (Rotation :type "Rotator Structure") (Distance :type "Float (double-precision)"))
  (returns (`New Location` :type "Vector Structure"))
  (return (+ Center (* (`KismetMathLibrary.GetForwardVector` Rotation) Distance))))

(fn `UserConstructionScript`)