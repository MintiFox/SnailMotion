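; PlayerCameraTarget is a camera target actor that the game mode's Cam can start on or blend to.
; If flagged StartingCamera, it registers as the current target after a zero-length delay on BeginPlay.
; Activate runs a timeline at a given play rate, driving Cam's blend percent through a curve, then becomes the current target.
; SetStartingCamera clears the flag on all targets before setting its own, keeping one start camera.
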(event `self.ReceiveBeginPlay`
  (if (`self.Starting Camera`)
    (`KismetSystemLibrary.Delay` 0.0)
    (bind _asbp_game_mode_base (cast `/Game/Blueprints/BP-GameMode_Base` (`GameplayStatics.GetGameMode`)))
    (set `/Game/Blueprints/Camera/PlayerLevelCamera.CurrentTarget` self (`/Game/Blueprints/BP-GameMode_Base.Cam` _asbp_game_mode_base))))

(event `/Game/Blueprints/Interfaces/IActivatable.Activate`
  (params (Float :type "Float (double-precision)"))
  (`TimelineComponent.SetPlayRate` (`self.CamTransitionTimeline`) Float)
  (bind _asbp_game_mode_base (cast `/Game/Blueprints/BP-GameMode_Base` (`GameplayStatics.GetGameMode`)))
  (bind _cam (`/Game/Blueprints/BP-GameMode_Base.Cam` _asbp_game_mode_base))
  (set `/Game/Blueprints/Camera/PlayerLevelCamera.BlendTarget` self _cam)
  (bind (_direction _t) (`Timeline|CamTransitionTimeline` :!via `PlayFromStart`)
    (:`Update`
      (set `/Game/Blueprints/Camera/PlayerLevelCamera.BlendPercent` (`CurveFloat.GetFloatValue` (`self.ActivateTransitionCruve`) _t) _cam))
    (:`Finished`
      (set `/Game/Blueprints/Camera/PlayerLevelCamera.CurrentTarget` self _cam)
      (set `/Game/Blueprints/Camera/PlayerLevelCamera.BlendTarget` null _cam))))

(fn `Set Starting Camera`
  (bind _outactors (`GameplayStatics.GetAllActorsOfClass` "PlayerCameraTarget_C"))
  (for _array_element _outactors
    (bind _asplayer_camera_target (cast `/Game/Blueprints/Camera/PlayerCameraTarget` _array_element))
    (set `/Game/Blueprints/Camera/PlayerCameraTarget.Starting Camera` false _asplayer_camera_target))
  (set `self.Starting Camera` true))

(fn `UserConstructionScript`)