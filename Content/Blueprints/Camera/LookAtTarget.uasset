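; LookAtTarget is a component that smoothly rotates its owning camera actor to face a target, optionally the player pawn.
; If the target is flagged as the player, it fetches the pawn shortly after BeginPlay.
; Each tick it aims from the owner's CameraComponent and interpolates the owner's rotation at a set speed.
; For BP_PlayerBase targets flagged as player, it aims at LastGroundedHeight instead of current Z, so jumps don't tilt the view.
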(event `self.ReceiveBeginPlay`
  (`KismetSystemLibrary.Delay` 0.2)
  (if (`self.TargetisPlayer`)
    (set `self.Target` (`GameplayStatics.GetPlayerPawn` 0))))

(event `self.ReceiveTick`
  (params (DeltaSeconds :type "Float (single-precision)"))
  (bind (_returnvalue_x _returnvalue_y) (`KismetMathLibrary.BreakVector` (`Actor.K2_GetActorLocation` (`self.Target`))))
  (if (`KismetSystemLibrary.IsValid` (`self.Target`))
    (if (`self.TargetisPlayer`)
      (bind _asbp_player_base (cast `/Game/Blueprints/BP_PlayerBase` (`self.Target`))
        (:`then`
          (set `self.TargetRot` (`KismetMathLibrary.FindLookAtRotation` (`SceneComponent.K2_GetComponentLocation` (`Actor.GetComponentByClass` (`self.GetOwner`) "/Script/Engine.CameraComponent")) (`KismetMathLibrary.MakeVector` _returnvalue_x _returnvalue_y (`/Game/Blueprints/BP_PlayerBase.LastGroundedHeight` _asbp_player_base)))))
        (:`CastFailed`
          (set `self.TargetRot` (`KismetMathLibrary.FindLookAtRotation` (`SceneComponent.K2_GetComponentLocation` (`Actor.GetComponentByClass` (`self.GetOwner`) "/Script/Engine.CameraComponent")) (`Actor.K2_GetActorLocation` (`self.Target`))) :!label _label)))
      (else
        (goto _label)))
    (`Actor.K2_SetActorRotation` (`self.GetOwner`) (`KismetMathLibrary.RInterpTo` (`Actor.K2_GetActorRotation` (`self.GetOwner`)) (`self.TargetRot`) DeltaSeconds (`self.Speed`)) false)))