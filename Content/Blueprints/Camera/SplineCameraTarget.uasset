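; Spline-constrained camera target that follows the player along a two-level rail, a Range spline that slides along a Path spline.
; Each tick the offset player position places Range at its closest point on Path, then TargetCam at the closest point on Range.
; Height tracks the player's last grounded height, and flags let each level inherit spline rotation.
; AutoGetOffset derives CamOffset by tracing along the camera's forward vector.
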(event `self.ReceiveBeginPlay`
  (`parent.ReceiveBeginPlay`)
  (bind _asbp_player_base (cast `/Game/Blueprints/BP_PlayerBase` (`GameplayStatics.GetPlayerPawn` 0)))
  (set `self.PlayerRef` _asbp_player_base)
  (set `self.UsableOffset` (- (`SceneComponent.K2_GetComponentLocation` (`self.TargetCam`)) (`KismetMathLibrary.TransformLocation` (`self.GetTransform`) (`self.CamOffset`))))
  (set `self.RangeStartRot` (`KismetMathLibrary.NormalizedDeltaRotator` (`SceneComponent.K2_GetComponentRotation` (`self.Range`)) (`SplineComponent.GetRotationAtTime` (`self.Path`) 0.0 "World" true)))
  (set `self.CamStartRot` (`KismetMathLibrary.NormalizedDeltaRotator` (`SceneComponent.K2_GetComponentRotation` (`self.TargetCam`)) (`SplineComponent.GetRotationAtTime` (`self.Range`) 0.0 "World" true))))

(event `self.ReceiveTick`
  (params (DeltaSeconds :type "Float (single-precision)"))
  (bind (_returnvalue_x _returnvalue_y _returnvalue_z) (`KismetMathLibrary.BreakVector` (`KismetMathLibrary.TransformLocation` (`self.GetTransform`) (`self.CamOffset`))))
  (`parent.ReceiveTick` DeltaSeconds)
  (if (`KismetSystemLibrary.IsValid` (`self.PlayerRef`))
    (bind _closestpoint (`self.GetClosestPoint` (+ (`self.UsableOffset`) (`self.K2_GetActorLocation` (`self.PlayerRef`)))))
    (`SceneComponent.K2_SetWorldTransform` (`self.TargetCam`) (`KismetMathLibrary.MakeTransform` (- (.location _closestpoint) (`KismetMathLibrary.MakeVector` 0.0 0.0 (- _returnvalue_z (`/Game/Blueprints/BP_PlayerBase.LastGroundedHeight` (`self.PlayerRef`))))) (`KismetMathLibrary.SelectRotator` (`KismetMathLibrary.ComposeRotators` (`self.CamStartRot`) (.rotation _closestpoint)) (`SceneComponent.K2_GetComponentRotation` (`self.TargetCam`)) (`self.RotCamWithRange`))) false false)))

(fn `AutoGetOffset`
  (bind _targetcam (`self.TargetCam`))
  (bind _returnvalue (`SceneComponent.K2_GetComponentLocation` _targetcam))
  (bind _outhit (`KismetSystemLibrary.LineTraceSingle` _returnvalue (+ _returnvalue (* (`SceneComponent.GetForwardVector` _targetcam) 5000.0)) "TraceTypeQuery1"))
  (set `self.CamOffset` (`KismetMathLibrary.InverseTransformLocation` (`self.GetTransform`) (`.Location` (`GameplayStatics.BreakHitResult` _outhit)))))

(fn `GetClosestPoint`
  (params (ReferencePoint :type "Vector Structure"))
  (returns (ClosestPoint :type "Transform Structure"))
  (locals (refPoint :type "Vector Structure"))
  (bind _range (`self.Range`))
  (bind (_returnvalue_location _returnvalue_rotation) (`KismetMathLibrary.BreakTransform` (`SplineComponent.GetTransformAtTime` (`self.Path`) (`SplineComponent.FindInputKeyClosestToWorldLocation` (`self.Path`) (`local.refPoint`)) "World" true false)))
  (set `local.refPoint` ReferencePoint)
  (`SceneComponent.K2_SetWorldTransform` _range (`KismetMathLibrary.MakeTransform` _returnvalue_location (`KismetMathLibrary.SelectRotator` (`KismetMathLibrary.ComposeRotators` (`self.RangeStartRot`) _returnvalue_rotation) (`SceneComponent.K2_GetComponentRotation` _range) (`self.RotRangeWithPath`))) false false)
  (return (`SplineComponent.GetTransformAtTime` (`self.Range`) (`SplineComponent.FindInputKeyClosestToWorldLocation` (`self.Range`) (`local.refPoint`)) "World" true false)))

(fn `UserConstructionScript`
  (`parent.UserConstructionScript`))