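; A camera trigger zone that switches the game mode's shared camera to CamA when the player enters and to CamB when they leave.
; A zero TransitionSpeed triggers a jump cut; otherwise a timeline at that play rate drives the blend percent through a curve.
; The timeline reverses mid-blend if the player crosses back, then settles on the nearer target.
; The construction script sizes and offsets the box from BoxSize, anchoring it at a corner.
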(event `self.ReceiveBeginPlay`
  (`KismetSystemLibrary.Delay` 0.0)
  (bind _asbp_game_mode_base (cast `/Game/Blueprints/BP-GameMode_Base` (`GameplayStatics.GetGameMode`)))
  (set `self.Cam` (`/Game/Blueprints/BP-GameMode_Base.Cam` _asbp_game_mode_base)))

(event `self.Box.OnComponentBeginOverlap`
  (params (OverlappedComponent :type "PrimitiveComponent Object Reference") (OtherActor :type "Actor Object Reference") (OtherComp :type "PrimitiveComponent Object Reference") (OtherBodyIndex :type Integer) (bFromSweep :type Boolean) (SweepResult :type "HitResult Structure (by ref)"))
  (cast `/Game/Blueprints/BP_PlayerBase` OtherActor)
  (if (== (`self.TransitionSpeed`) 0.0)
    (set `/Game/Blueprints/Camera/PlayerLevelCamera.CurrentTarget` (`self.CamA`) (`self.Cam`))
    (set `/Game/Blueprints/Camera/PlayerLevelCamera.BlendTarget` null (`self.Cam`))
    (`KismetSystemLibrary.Delay` 0.0)
    (`/Game/Blueprints/Camera/PlayerLevelCamera.JumpCut` (`self.Cam`))
    (else
      (`TimelineComponent.SetPlayRate` (`self.CamTransitionTimeline`) (`self.TransitionSpeed`))
      (`|ExecutionSequence`
        (:`then_0`
          (set `/Game/Blueprints/Camera/PlayerLevelCamera.CurrentTarget` (`self.CamA`) (`self.Cam`) :!label _label)
          (set `/Game/Blueprints/Camera/PlayerLevelCamera.BlendTarget` (`self.CamB`) (`self.Cam`)))
        (:`then_1`
          (if (`TimelineComponent.IsPlaying` (`self.CamTransitionTimeline`))
            (bind (_direction _t) (`Timeline|CamTransitionTimeline` :!via `Reverse` :!label _label_2)
              (:`Update`
                (set `/Game/Blueprints/Camera/PlayerLevelCamera.BlendPercent` (`CurveFloat.GetFloatValue` (`self.CamTransitionCurve`) _t) (`self.Cam`)))
              (:`Finished`
                (set `/Game/Blueprints/Camera/PlayerLevelCamera.CurrentTarget` (select `bool` (> _t 0.5) :`false` (`self.CamA`) :`true` (`self.CamB`)) (`self.Cam`))
                (set `/Game/Blueprints/Camera/PlayerLevelCamera.BlendTarget` null (`self.Cam`))))
            (else
              (goto _label_2 :!via `ReverseFromEnd`))))))))

(event `self.Box.OnComponentEndOverlap`
  (params (OverlappedComponent :type "PrimitiveComponent Object Reference") (OtherActor :type "Actor Object Reference") (OtherComp :type "PrimitiveComponent Object Reference") (OtherBodyIndex :type Integer))
  (cast `/Game/Blueprints/BP_PlayerBase` OtherActor)
  (if (== (`self.TransitionSpeed`) 0.0)
    (set `/Game/Blueprints/Camera/PlayerLevelCamera.CurrentTarget` (`self.CamB`) (`self.Cam`))
    (set `/Game/Blueprints/Camera/PlayerLevelCamera.BlendTarget` null (`self.Cam`))
    (`KismetSystemLibrary.Delay` 0.0)
    (`/Game/Blueprints/Camera/PlayerLevelCamera.JumpCut` (`self.Cam`))
    (else
      (`TimelineComponent.SetPlayRate` (`self.CamTransitionTimeline`) (`self.TransitionSpeed`))
      (`|ExecutionSequence`
        (:`then_0`
          (goto _label))
        (:`then_1`
          (if (`TimelineComponent.IsPlaying` (`self.CamTransitionTimeline`))
            (goto _label_2)
            (else
              (goto _label_2 :!via `PlayFromStart`))))))))

(fn `UserConstructionScript`
  (`BoxComponent.SetBoxExtent` (`self.Box`) (* (`self.BoxSize`) 0.5) true)
  (`SceneComponent.K2_SetRelativeLocation` (`self.Box`) (* (`self.BoxSize`) 0.5) false false))