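; Camera trigger volume that switches the player's view between two targets, A and B, as the player crosses it.
; Two overlapping boxes track the Player-tagged actor, and leaving one while still inside the other gives the crossing direction.
; PlayerCamera targets are enabled with a per-direction transition time and the opposite one disabled, while other actors get a cubic view-target blend.
; The construction script draws colored debug arrows to both targets.
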(event `self.ReceiveBeginPlay`
  (`KismetSystemLibrary.Delay` 0.0))

(event `self.Hitbox2.OnComponentBeginOverlap`
  (params (OverlappedComponent :type "PrimitiveComponent Object Reference") (OtherActor :type "Actor Object Reference") (OtherComp :type "PrimitiveComponent Object Reference") (OtherBodyIndex :type Integer) (bFromSweep :type Boolean) (SweepResult :type "HitResult Structure (by ref)"))
  (if (`self.ActorHasTag` OtherActor "Player")
    (set `self.Box2Overlap` true)))

(event `self.Hitbox2.OnComponentEndOverlap`
  (params (OverlappedComponent :type "PrimitiveComponent Object Reference") (OtherActor :type "Actor Object Reference") (OtherComp :type "PrimitiveComponent Object Reference") (OtherBodyIndex :type Integer))
  (if (`self.ActorHasTag` OtherActor "Player")
    (set `self.Box2Overlap` false)
    ;[1 1 1] Going from 2 to 1
    (if (`self.Box1Overlap`)
      (bind _asplayer_camera (cast `/Game/Blueprints/Camera/PlayerCamera` (`self.View Target A`))
        (:`then`
          (`/Game/Blueprints/Camera/PlayerCamera.EnableCam` _asplayer_camera (`self.TransitionTimeA`)))
        (:`CastFailed`
          (`PlayerController.SetViewTargetWithBlend` (`GameplayStatics.GetPlayerController` 0) (`self.View Target A`) (`self.TransitionTimeA`) "VTBlend_Cubic" 1.0 false)))
      (bind _asplayer_camera_2 (cast `/Game/Blueprints/Camera/PlayerCamera` (`self.View Target B`)))
      (`/Game/Blueprints/Camera/PlayerCamera.DisableCam` _asplayer_camera_2))))

(event `self.CollisionComponent.OnComponentBeginOverlap`
  (params (OverlappedComponent :type "PrimitiveComponent Object Reference") (OtherActor :type "Actor Object Reference") (OtherComp :type "PrimitiveComponent Object Reference") (OtherBodyIndex :type Integer) (bFromSweep :type Boolean) (SweepResult :type "HitResult Structure (by ref)"))
  (if (`self.ActorHasTag` OtherActor "Player")
    (set `self.Box1Overlap` true)))

(event `self.CollisionComponent.OnComponentEndOverlap`
  (params (OverlappedComponent :type "PrimitiveComponent Object Reference") (OtherActor :type "Actor Object Reference") (OtherComp :type "PrimitiveComponent Object Reference") (OtherBodyIndex :type Integer))
  (if (`self.ActorHasTag` OtherActor "Player")
    (set `self.Box1Overlap` false)
    ;[1 1 1] Going from 1 to 2
    (if (`self.Box2Overlap`)
      (bind _asplayer_camera (cast `/Game/Blueprints/Camera/PlayerCamera` (`self.View Target B`))
        (:`then`
          (`/Game/Blueprints/Camera/PlayerCamera.EnableCam` _asplayer_camera (`self.TransitionTimeB`)))
        (:`CastFailed`
          (`PlayerController.SetViewTargetWithBlend` (`GameplayStatics.GetPlayerController` 0) (`self.View Target B`) (`self.TransitionTimeB`) "VTBlend_Cubic" 1.0 false)))
      (bind _asplayer_camera_2 (cast `/Game/Blueprints/Camera/PlayerCamera` (`self.View Target A`)))
      (`/Game/Blueprints/Camera/PlayerCamera.DisableCam` _asplayer_camera_2))))

(fn `UserConstructionScript`
  (if (`KismetSystemLibrary.IsValid` (`self.View Target A`))
    (`KismetSystemLibrary.DrawDebugArrow` (`SceneComponent.K2_GetComponentLocation` (`self.A`)) (`self.K2_GetActorLocation` (`self.View Target A`)) 0.0 (struct :`R` 1.0 :`G` 0.317647 :`B` 0.352941 :`A` 1.0) 0.5 10.0))
  (if (`KismetSystemLibrary.IsValid` (`self.View Target B`))
    (`KismetSystemLibrary.DrawDebugArrow` (`SceneComponent.K2_GetComponentLocation` (`self.B`)) (`self.K2_GetActorLocation` (`self.View Target B`)) 0.0 (struct :`R` 0.098039 :`G` 0.152941 :`B` 0.737255 :`A` 1.0) 0.5 10.0)))