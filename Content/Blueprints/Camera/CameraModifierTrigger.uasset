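; Camera trigger that switches the player's view between two targets, A and B, using two overlapping hitboxes to detect crossing direction.
; Leaving one box while still inside the other blends to that side's target with its own transition time.
; PlayerCamera targets use their own enable and disable calls, while others use a cubic view-target blend.
; After BeginPlay, CamOnSpline targets are replaced by their inner Cam.
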(event `self.ReceiveBeginPlay`
  (`KismetSystemLibrary.Delay` 0.0)
  (bind _ascam_on_spline (cast `/Game/Blueprints/Camera/CamOnSpline` (`self.View Target A`))
    (:`then`
      (set `self.View Target A` (`/Game/Blueprints/Camera/CamOnSpline.Cam` _ascam_on_spline)))
    (:`CastFailed`
      _))
  (bind _ascam_on_spline_2 (cast `/Game/Blueprints/Camera/CamOnSpline` (`self.View Target B`)))
  (set `self.View Target B` (`/Game/Blueprints/Camera/CamOnSpline.Cam` _ascam_on_spline_2)))

(event `self.Hitbox2.OnComponentBeginOverlap`
  (params (OverlappedComponent :type "PrimitiveComponent Object Reference") (OtherActor :type "Actor Object Reference") (OtherComp :type "PrimitiveComponent Object Reference") (OtherBodyIndex :type Integer) (bFromSweep :type Boolean) (SweepResult :type "HitResult Structure (by ref)"))
  (set `self.Box2Overlap` true))

(event `self.Hitbox2.OnComponentEndOverlap`
  (params (OverlappedComponent :type "PrimitiveComponent Object Reference") (OtherActor :type "Actor Object Reference") (OtherComp :type "PrimitiveComponent Object Reference") (OtherBodyIndex :type Integer))
  (set `self.Box2Overlap` false)
  ;[1 1 1] Going from 2 to 1
  (if (`self.Box1Overlap`)
    (bind _asplayer_camera (cast `/Game/Blueprints/Camera/PlayerCamera` (`self.View Target A`))
      (:`then`
        (`/Game/Blueprints/Camera/PlayerCamera.EnableCam` _asplayer_camera (`self.TransitionTimeA`)))
      (:`CastFailed`
        (`PlayerController.SetViewTargetWithBlend` (`GameplayStatics.GetPlayerController` 0) (`self.View Target A`) (`self.TransitionTimeA`) "VTBlend_Cubic" 1.0 false)))
    (bind _asplayer_camera_2 (cast `/Game/Blueprints/Camera/PlayerCamera` (`self.View Target B`)))
    (`/Game/Blueprints/Camera/PlayerCamera.DisableCam` _asplayer_camera_2)))

(event `self.CollisionComponent.OnComponentBeginOverlap`
  (params (OverlappedComponent :type "PrimitiveComponent Object Reference") (OtherActor :type "Actor Object Reference") (OtherComp :type "PrimitiveComponent Object Reference") (OtherBodyIndex :type Integer) (bFromSweep :type Boolean) (SweepResult :type "HitResult Structure (by ref)"))
  (set `self.Box1Overlap` true))

(event `self.CollisionComponent.OnComponentEndOverlap`
  (params (OverlappedComponent :type "PrimitiveComponent Object Reference") (OtherActor :type "Actor Object Reference") (OtherComp :type "PrimitiveComponent Object Reference") (OtherBodyIndex :type Integer))
  (set `self.Box1Overlap` false)
  ;[1 1 1] Going from 1 to 2
  (if (`self.Box2Overlap`)
    (bind _asplayer_camera (cast `/Game/Blueprints/Camera/PlayerCamera` (`self.View Target B`))
      (:`then`
        (`/Game/Blueprints/Camera/PlayerCamera.EnableCam` _asplayer_camera (`self.TransitionTimeB`)))
      (:`CastFailed`
        (`PlayerController.SetViewTargetWithBlend` (`GameplayStatics.GetPlayerController` 0) (`self.View Target B`) (`self.TransitionTimeB`) "VTBlend_Cubic" 1.0 false)))
    (bind _asplayer_camera_2 (cast `/Game/Blueprints/Camera/PlayerCamera` (`self.View Target A`)))
    (`/Game/Blueprints/Camera/PlayerCamera.DisableCam` _asplayer_camera_2)))

(fn `UserConstructionScript`)