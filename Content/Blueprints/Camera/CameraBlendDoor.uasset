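; CameraBlendDoor is a box trigger that blends the game mode's camera between CamA and CamB as the player moves through it.
; The construction script sizes the box from BoxSize and offsets markers A and B to its ends along local X.
; While overlapped, Tick maps the player's normalized local X position through TransitionCurve into the camera's BlendPercent.
; On exit, the nearer end's camera becomes the current target and the blend target is cleared.
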(event `self.ReceiveBeginPlay`
  (`KismetSystemLibrary.Delay` 0.0)
  (bind _asbp_game_mode_base (cast `/Game/Blueprints/BP-GameMode_Base` (`GameplayStatics.GetGameMode`)))
  (set `self.Cam` (`/Game/Blueprints/BP-GameMode_Base.Cam` _asbp_game_mode_base)))

(event `self.ReceiveActorBeginOverlap`
  (params (OtherActor :type "Actor Object Reference"))
  (cast `/Game/Blueprints/BP_PlayerBase` OtherActor)
  (set `/Game/Blueprints/Camera/PlayerLevelCamera.CurrentTarget` (`self.CamA`) (`self.Cam`))
  (set `/Game/Blueprints/Camera/PlayerLevelCamera.CurrentTarget` (`self.CamA`) (`self.Cam`))
  (set `/Game/Blueprints/Camera/PlayerLevelCamera.BlendTarget` (`self.CamB`) (`self.Cam`))
  (set `self.PlayerOverlapping` true))

(event `self.ReceiveActorEndOverlap`
  (params (OtherActor :type "Actor Object Reference"))
  (cast `/Game/Blueprints/BP_PlayerBase` OtherActor)
  (set `self.PlayerOverlapping` false)
  (bind _t (`self.Generate T`))
  (set `/Game/Blueprints/Camera/PlayerLevelCamera.CurrentTarget` (select `bool` (> _t 0.5) :`false` (`self.CamA`) :`true` (`self.CamB`)) (`self.Cam`))
  (set `/Game/Blueprints/Camera/PlayerLevelCamera.BlendTarget` null (`self.Cam`)))

(event `self.ReceiveTick`
  (params (DeltaSeconds :type "Float (single-precision)"))
  (if (`self.PlayerOverlapping`)
    (bind _t (`self.Generate T`))
    (set `/Game/Blueprints/Camera/PlayerLevelCamera.BlendPercent` (`CurveFloat.GetFloatValue` (`self.TransitionCurve`) _t) (`self.Cam`))))

(fn `Generate T`
  (returns (t :type "Float (double-precision)"))
  (bind _returnvalue_x (`KismetMathLibrary.BreakVector` (`KismetMathLibrary.InverseTransformLocation` (`self.GetTransform`) (`self.K2_GetActorLocation` (`GameplayStatics.GetPlayerPawn` 0)))))
  (return (`KismetMathLibrary.FClamp` (`KismetMathLibrary.NormalizeToRange` _returnvalue_x 0.0 (`KismetMathLibrary.Vector_Distance` (`SceneComponent.RelativeLocation` (`self.A`)) (`SceneComponent.RelativeLocation` (`self.B`)))))))

(fn `UserConstructionScript`
  (bind (_returnvalue_x _returnvalue_y _returnvalue_z) (`KismetMathLibrary.BreakVector` (* (`BoxComponent.GetScaledBoxExtent` (`self.Box`)) 1.0)))
  (bind (_returnvalue_x_2 _returnvalue_y_2 _returnvalue_z_2) (`KismetMathLibrary.BreakVector` (* (`BoxComponent.GetScaledBoxExtent` (`self.Box`)) 1.0)))
  (`BoxComponent.SetBoxExtent` (`self.Box`) (* (`self.BoxSize`) 0.5) true)
  (`SceneComponent.K2_SetRelativeLocation` (`self.Box`) (* (`self.BoxSize`) 0.5) false false)
  (`SceneComponent.K2_AddLocalOffset` (`self.A`) (`KismetMathLibrary.MakeVector` 0.0 _returnvalue_y_2 _returnvalue_z_2) false false)
  (`SceneComponent.K2_AddLocalOffset` (`self.B`) (`KismetMathLibrary.MakeVector` (* _returnvalue_x 2.0) _returnvalue_y _returnvalue_z) false false))