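; A camera point of interest that pulls the game mode's player camera toward itself as the player approaches.
; Entering the outer sphere sets it as the camera's BlendTarget, optionally only when the camera's current target is in EffectOnlyTheseCams; leaving clears it.
; While overlapping, Tick maps player distance to BlendPercent, from MaxStrength at the inner sphere to zero at the outer.
; The construction script drives both radii from X-only vectors.
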(event `self.ReceiveBeginPlay`
  (`parent.ReceiveBeginPlay`)
  (`KismetSystemLibrary.Delay` 0.0)
  (bind _asbp_game_mode_base (cast `/Game/Blueprints/BP-GameMode_Base` (`GameplayStatics.GetGameMode`)))
  (set `self.PlayerCam` (`/Game/Blueprints/BP-GameMode_Base.Cam` _asbp_game_mode_base)))

(event `self.OuterSphere.OnComponentBeginOverlap`
  (params (OverlappedComponent :type "PrimitiveComponent Object Reference") (OtherActor :type "Actor Object Reference") (OtherComp :type "PrimitiveComponent Object Reference") (OtherBodyIndex :type Integer) (bFromSweep :type Boolean) (SweepResult :type "HitResult Structure (by ref)"))
  (bind _asbp_player_base (cast `/Game/Blueprints/BP_PlayerBase` OtherActor))
  (if (> (`KismetArrayLibrary.Array_Length` (`self.EffectOnlyTheseCams`)) 0)
    (for _array_element (`self.EffectOnlyTheseCams`)
      (if (== (`/Game/Blueprints/Camera/PlayerLevelCamera.CurrentTarget` (`self.PlayerCam`)) _array_element)
        (set `self.InAllowedCam` true)))
    (if (`self.InAllowedCam`)
      (set `self.isOverlapping` true :!label _label)
      (set `self.PlayerRef` _asbp_player_base)
      (set `/Game/Blueprints/Camera/PlayerLevelCamera.BlendTarget` self (`self.PlayerCam`)))
    (else
      (goto _label))))

(event `self.OuterSphere.OnComponentEndOverlap`
  (params (OverlappedComponent :type "PrimitiveComponent Object Reference") (OtherActor :type "Actor Object Reference") (OtherComp :type "PrimitiveComponent Object Reference") (OtherBodyIndex :type Integer))
  (cast `/Game/Blueprints/BP_PlayerBase` OtherActor)
  (if (> (`KismetArrayLibrary.Array_Length` (`self.EffectOnlyTheseCams`)) 0)
    (if (`self.InAllowedCam`)
      (set `self.isOverlapping` false :!label _label_2)
      (set `/Game/Blueprints/Camera/PlayerLevelCamera.BlendTarget` null (`self.PlayerCam`))
      (set `self.InAllowedCam` false))
    (else
      (goto _label_2))))

(event `self.ReceiveTick`
  (params (DeltaSeconds :type "Float (single-precision)"))
  (`parent.ReceiveTick` DeltaSeconds)
  (if (`self.isOverlapping`)
    (bind _t (`self.GenerateT` (`self.K2_GetActorLocation` (`self.PlayerRef`))))
    (set `/Game/Blueprints/Camera/PlayerLevelCamera.BlendPercent` _t (`self.PlayerCam`))))

(fn `GenerateT`
  (params (Position :type "Vector Structure"))
  (returns (T :type "Float (double-precision)"))
  (return (`KismetMathLibrary.MapRangeClamped` (`KismetMathLibrary.Vector_Distance` Position (`SceneComponent.K2_GetComponentLocation` (`self.OuterSphere`))) (`SphereComponent.SphereRadius` (`self.InnerSphere`)) (`SphereComponent.SphereRadius` (`self.OuterSphere`)) (`self.MaxStrength`))))

(fn `UserConstructionScript`
  (bind _outersphereradius_x (`KismetMathLibrary.BreakVector` (`self.OuterSphereRadius`)))
  (bind _innersphereradius_x (`KismetMathLibrary.BreakVector` (`self.InnerSphereRadius`)))
  (bind _outersphereradius_x_2 (`KismetMathLibrary.BreakVector` (`self.OuterSphereRadius`)))
  (bind _innersphereradius_x_2 (`KismetMathLibrary.BreakVector` (`self.InnerSphereRadius`)))
  (`SphereComponent.SetSphereRadius` (`self.OuterSphere`) _outersphereradius_x false)
  (`SphereComponent.SetSphereRadius` (`self.InnerSphere`) _innersphereradius_x false)
  (set `self.OuterSphereRadius` (`KismetMathLibrary.MakeVector` _outersphereradius_x_2))
  (set `self.InnerSphereRadius` (`KismetMathLibrary.MakeVector` _innersphereradius_x_2)))