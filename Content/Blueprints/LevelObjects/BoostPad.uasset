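; BP BoostPad is a level object that sends the player rolling at a boosted speed along the pad's direction.
; On overlap with a BP_PlayerBase, it turns the player to the mesh's right vector, changes their state and sets a roll speed with a decay time.
; It also fires its Activator to trigger all linked activatables.
; An older launch and input-stop approach remains unconnected.
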(event `self.ReceiveActorBeginOverlap`
  (params (OtherActor :type "Actor Object Reference"))
  (bind _asbp_player_base (cast `/Game/Blueprints/BP_PlayerBase` OtherActor))
  (bind _output_get (set `self.Player` _asbp_player_base))
  (`/Game/Blueprints/BP_PlayerBase.SetForward` _output_get (`SceneComponent.GetRightVector` (`self.StaticMeshComponent`)))
  (`/Game/Blueprints/Components/Activator.ActivateAllActivatables` (`self.Activator`))
  (`/Game/Blueprints/BP_PlayerBase.Set State` (`self.Player`) "NewEnumerator1")
  (`/Game/Blueprints/BP_PlayerBase.SetRollSpeed` (`self.Player`) (`self.Speed`) (`self.Decay Time`)))

(fn `UserConstructionScript`)