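; Soda bottle fountain level object whose column cyclically rises and falls, launching players who overlap it along the actor's up axis.
; A timeline drives column height between holds, preceded by a warning that shakes the optional cap or plays particles.
; Shelled players lose roll speed and get a kick, and Tick keeps pushing any overlapping player.
; The construction script toggles cap and pretzel grid and tints soda and bottle materials.
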(event `self.ReceiveBeginPlay`
  (`KismetSystemLibrary.Delay` (`self.TimeOffset`))
  (set `self.StartPos` (`SceneComponent.RelativeLocation` (`self.Collumn`)))
  (`self.MoveColumn` (`self.Up`))
  (if (not (`self.Grid`))
    (`ActorComponent.K2_DestroyComponent` (`self.PretzelGrid`)))
  (if (not (`self.BottleCap`))
    (`ActorComponent.K2_DestroyComponent` (`self.Cap`))
    (`ActorComponent.K2_DestroyComponent` (`self.CapCollider`))))

(event `MoveColumn`
  (params (Up :type Boolean))
  (bind _up (`self.Up`))
  (if Up
    (if (`self.BottleCap`)
      (set `self.bottle start location` (`SceneComponent.K2_GetComponentLocation` (`self.Cap`)))
      (else
        (`ActorComponent.Activate` (`self.Particles`) false)))
    (`TimelineComponent.SetNewTime` (`self.AnticipationTime`) (- 5.0 (`self.WarningTime`)))
    (`Timeline|AnticipationTime`
      (:`Update`
        (if (`self.BottleCap`)
          (bind _newlocation (`self.Shake` (`self.bottle start location`) 5.0))
          (`SceneComponent.K2_SetWorldLocation` (`self.Cap`) _newlocation false false)))
      (:`Finished`
        (if (`self.BottleCap`)
          (`SceneComponent.K2_SetWorldLocation` (`self.Cap`) (`self.bottle start location`) false false))
        (`ActorComponent.Deactivate` (`self.Particles`))
        ;[1 1 1] Go Up
        (set `PrimitiveComponent.bGenerateOverlapEvents` true (`self.Collumn`))
        (`TimelineComponent.SetPlayRate` (`self.FlowUp`) (`self.UpSpeed`))
        (bind (_direction _height) (`Timeline|FlowUp` :!via `PlayFromStart` :!label _label)
          (:`Update`
            (`SceneComponent.K2_SetRelativeLocation` (`self.Collumn`) (`KismetMathLibrary.MakeVector` 0.0 0.0 (+ (* _height (`self.Height`)) (.z (`self.StartPos`)))) false false))
          (:`Finished`
            (if (not (`self.Up`))
              (set `PrimitiveComponent.bGenerateOverlapEvents` false (`self.Collumn`)))
            ;[1 1 1] Reset Timer
            (if (`self.Up`)
              (`KismetSystemLibrary.Delay` (`self.UpHoldTime`))
              (else
                (`KismetSystemLibrary.Delay` (`self.DownHoldTime`))))
            (set `self.Up` (not _up))
            (`self.MoveColumn` _up)))))
    (else
      (`ActorComponent.Deactivate` (`self.Particles`))
      (`TimelineComponent.SetPlayRate` (`self.FlowUp`) (`self.DownSpeed`))
      (goto _label :!via `ReverseFromEnd`))))

(event `self.ReceiveActorBeginOverlap`
  (params (OtherActor :type "Actor Object Reference"))
  ;[1 1 1] On overlap
  (bind _asbp_player_base (cast `/Game/Blueprints/BP_PlayerBase` OtherActor))
  (bind _output_get (set `self.OverlappedPlayer` _asbp_player_base))
  (if (`|EnumEquality` (`/Game/Blueprints/BP_PlayerBase.MovementState` _output_get) "NewEnumerator1")
    (`/Game/Blueprints/BP_PlayerBase.SetRollSpeed` (`self.OverlappedPlayer`) 0.0 0.0)
    ;[1 1 1] If in shell, launch player
    (`Character.LaunchCharacter` (`self.OverlappedPlayer`) (* (`KismetMathLibrary.TransformDirection` (`self.GetTransform`) (0.0 0.0 1.0)) (`self.ForceKick`)) true true)
    (`KismetSystemLibrary.Delay` 0.2)
    (set `self.PlayerOverlapping` true)
    (else
      (set `self.PlayerOverlapping` true))))

(event `self.ReceiveActorEndOverlap`
  (params (OtherActor :type "Actor Object Reference"))
  ;[1 1 1] set flag on overlap end
  (set `self.PlayerOverlapping` false)
  (set `self.OverlappedPlayer` null))

(event `self.ReceiveTick`
  (params (DeltaSeconds :type "Float (single-precision)"))
  ;[1 1 1] Continue pushing player while in fountain
  (if (and (`self.PlayerOverlapping`) (`KismetSystemLibrary.IsValid` (`self.OverlappedPlayer`)))
    (`Character.LaunchCharacter` (`self.OverlappedPlayer`) (+ (0.0 0.0 0.0) (* (`KismetMathLibrary.TransformDirection` (`self.GetTransform`) (0.0 0.0 1.0)) (`self.ForceSustain`))) false false)))

(fn `Shake`
  (params (StartLocation :type "Vector Structure") (intensity :type "Float (double-precision)"))
  (returns (NewLocation :type "Vector Structure"))
  (return (+ StartLocation (* (`KismetMathLibrary.RandomUnitVector`) intensity))))

(fn `UserConstructionScript`
  (locals (NewLocalVar_0 :type "LinearColor Structure"))
  (bind _cap (`self.Cap`))
  (bind _pretzelgrid (`self.PretzelGrid`))
  ;[1 1 1] Adding bottle and pretzel grid
  (if (`self.BottleCap`)
    (`SceneComponent.SetVisibility` _cap true false)
    (else
      (`SceneComponent.SetVisibility` _cap false false)))
  (if (`self.Grid`)
    (`SceneComponent.SetVisibility` _pretzelgrid true false)
    (else
      (`SceneComponent.SetVisibility` _pretzelgrid false false)))
  ;[1 1 1] Setting up Colors
  (bind _returnvalue (`PrimitiveComponent.CreateDynamicMaterialInstance` (`self.Collumn`) 0 "/Game/Assets/Materials/Soda/Soda_Shaft.Soda_Shaft" "None"))
  (`MaterialInstanceDynamic.SetVectorParameterValue` _returnvalue "Color1" (`self.SodaColor1`))
  (`MaterialInstanceDynamic.SetVectorParameterValue` _returnvalue "Color2" (`self.SodaColor2`))
  (bind _returnvalue_2 (`PrimitiveComponent.CreateDynamicMaterialInstance` (`self.Collumn`) 2 "/Game/Assets/Materials/Soda/Soda_interior.Soda_interior" "None"))
  (`MaterialInstanceDynamic.SetVectorParameterValue` _returnvalue_2 "Color" (`self.SodaColor1`))
  (bind _returnvalue_3 (`PrimitiveComponent.CreateDynamicMaterialInstance` (`self.Collumn`) 1 "/Game/Assets/Materials/Soda/Soda_Cap.Soda_Cap" "None"))
  (`MaterialInstanceDynamic.SetVectorParameterValue` _returnvalue_3 "Color1" (`self.SodaColor1`))
  (`MaterialInstanceDynamic.SetVectorParameterValue` _returnvalue_3 "Color2" (`self.SodaColor2`))
  (bind _returnvalue_4 (`PrimitiveComponent.CreateDynamicMaterialInstance` (`self.StaticMeshComponent`) 0 "/Game/Assets/Materials/Bottle1.Bottle1" "None"))
  (`MaterialInstanceDynamic.SetVectorParameterValue` _returnvalue_4 "Color" (`self.BottleColor`)))