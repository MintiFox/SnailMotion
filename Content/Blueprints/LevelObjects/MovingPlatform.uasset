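; Moving platform level object that oscillates continuously between its placed location and an offset point.
; BeginPlay stores the start position and converts MoveToPos from a relative offset into a world-space target.
; Tick lerps between the two using a sine of time since creation scaled by Speed, so motion eases at both ends and begins from the midpoint.
; Location is set directly without sweeping, so the move ignores blocking collision.
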(event `self.ReceiveBeginPlay`
  (set `self.StartPos` (`self.K2_GetActorLocation`))
  (set `self.MoveToPos` (+ (`self.K2_GetActorLocation`) (`self.MoveToPos`))))

(event `self.ReceiveTick`
  (params (DeltaSeconds :type "Float (single-precision)"))
  (`self.K2_SetActorLocation` (`KismetMathLibrary.VLerp` (`self.StartPos`) (`self.MoveToPos`) (* (+ (`KismetMathLibrary.Sin` (* (`self.GetGameTimeSinceCreation`) (`self.Speed`))) 1.0) 0.5))))

(fn `UserConstructionScript`)