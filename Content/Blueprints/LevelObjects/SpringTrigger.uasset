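; SpringTrigger is a level object that launches the player along an arrow's forward direction when they overlap its box.
; It can zero the player's velocity first, then adds a launch scaled by SpringPower and moves the capsule to the arrow's location and yaw.
; An optional flag disables player zero's input for a set duration before restoring it.
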(event `self.ReceiveBeginPlay`)

(event `self.Box.OnComponentBeginOverlap`
  (params (OverlappedComponent :type "PrimitiveComponent Object Reference") (OtherActor :type "Actor Object Reference") (OtherComp :type "PrimitiveComponent Object Reference") (OtherBodyIndex :type Integer) (bFromSweep :type Boolean) (SweepResult :type "HitResult Structure (by ref)"))
  (bind _returnvalue (`GameplayStatics.GetPlayerController` 0))
  (bind _as_bp_player_base (`self.As BP Player Base`))
  (bind _arrow (`self.Arrow`))
  (bind (_returnvalue_roll _returnvalue_pitch _returnvalue_yaw) (`KismetMathLibrary.BreakRotator` (`SceneComponent.K2_GetComponentRotation` _arrow)))
  (bind _asbp_player_base (cast `/Game/Blueprints/BP_PlayerBase` OtherActor))
  (set `self.As BP Player Base` _asbp_player_base)
  (if (`self.StopVelocity?`)
    (set `MovementComponent.Velocity` (0.0 0.0 0.0) (`Character.CharacterMovement` _asbp_player_base)))
  (`Character.LaunchCharacter` _asbp_player_base (* (`SceneComponent.GetForwardVector` (`self.Arrow`)) (`self.SpringPower`)) false false)
  (if true
    (`SceneComponent.K2_SetWorldLocationAndRotation` (`Character.CapsuleComponent` _asbp_player_base) (`SceneComponent.K2_GetComponentLocation` _arrow) (`KismetMathLibrary.MakeRotator` 0.0 0.0 _returnvalue_yaw) false false))
  (if (`self.DisableMovement?`)
    (`self.DisableInput` _as_bp_player_base _returnvalue)
    (`KismetSystemLibrary.Delay` (`self.Duration`))
    (`self.EnableInput` _as_bp_player_base _returnvalue)))

(fn `UserConstructionScript`)