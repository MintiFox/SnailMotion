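; BoostRing is a level object that launches an overlapping player along the ring mesh's up axis.
; Launch velocity aims from the player toward a point scaled by Boost.Z, while gravity and input are briefly suspended and a dash montage plays.
; Overlap also fires linked activatables and runs a timeline that spins and scales the ring.
; The construction script keeps Boost Z-only and sizes a preview arrow from it.
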(event `self.ReceiveBeginPlay`
  (set `self.startScale` (`SceneComponent.K2_GetComponentScale` (`self.StaticMeshComponent`))))

(event `self.ReceiveActorBeginOverlap`
  (params (OtherActor :type "Actor Object Reference"))
  (bind (_boost_x _boost_y _boost_z) (`KismetMathLibrary.BreakVector` (`self.Boost`)))
  (bind _player (`self.player`))
  (bind _staticmeshcomponent (`self.StaticMeshComponent`))
  (bind (_returnvalue_x _returnvalue_y _returnvalue_z) (`KismetMathLibrary.BreakVector` (`SceneComponent.K2_GetComponentLocation` (`self.StaticMeshComponent`))))
  (bind _asbp_player_base (cast `/Game/Blueprints/BP_PlayerBase` OtherActor))
  (bind _output_get (set `self.player` _asbp_player_base))
  (`/Game/Blueprints/BP_PlayerBase.Set State` _output_get "NewEnumerator0")
  (`Character.LaunchCharacter` (`self.player`) (- (+ (* (`SceneComponent.GetUpVector` (`self.StaticMeshComponent`)) (* _boost_z 10.0)) (`self.K2_GetActorLocation`)) (`self.K2_GetActorLocation` (`self.player`))) true true)
  (`/Game/Blueprints/BP_PlayerBase.SetForward` _player (`SceneComponent.GetUpVector` (`self.StaticMeshComponent`)))
  (`Character.PlayAnimMontage` _player "/Game/Assets/Meshes/Drizzle/Drizzle_RingDash.Drizzle_RingDash" 1.5 "None")
  (set `/Game/Blueprints/BP_PlayerBase.LastGroundedHeight` _returnvalue_z (`self.player`))
  (`/Game/Blueprints/BP_PlayerBase.SetGravityScale` (`self.player`) 0.0 0.25)
  (`/Game/Blueprints/BP_PlayerBase.Stop Input` (`self.player`) 0.5)
  (`/Game/Blueprints/Components/Activator.ActivateAllActivatables` (`self.Activator`))
  (bind (_direction _float) (`Timeline|RingActivate` :!via `PlayFromStart`)
    (:`Update`
      (`SceneComponent.K2_AddLocalRotation` _staticmeshcomponent (`KismetMathLibrary.MakeRotator` 0.0 0.0 (* _float 2.0)) false false)
      (`SceneComponent.SetWorldScale3D` _staticmeshcomponent (+ (`self.startScale`) (* _float 0.25))))))

(fn `UserConstructionScript`
  (bind (_boost_x _boost_y _boost_z) (`KismetMathLibrary.BreakVector` (`self.Boost`)))
  (bind _output_get (set `self.Boost` (`KismetMathLibrary.MakeVector` 0.0 0.0 _boost_z)))
  (set `ArrowComponent.ArrowLength` (* (.z _output_get) 1.0) (`self.Arrow`)))