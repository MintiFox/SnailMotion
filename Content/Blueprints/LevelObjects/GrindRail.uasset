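; Spline-based grind rail of icing squeezed from a pouch, which connects overlapping players for grinding and fires activatables on attach and detach.
; GenerateRail builds spline mesh segments at construction or BeginPlay, each with an offset dynamic material for a staggered reveal.
; StartActive, Activate or ground-pound damage enables rail overlaps, squishes the pouch and runs the reveal as the tube cap follows the spline.
; Standing on the inactive pouch drives a smaller morph-target squish.
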(event `self.ReceiveBeginPlay`
  (set `self.startRot` (`SceneComponent.RelativeRotation` (`self.icing_Tube_Cap`)))
  (if (not (`self.GenerateRealtime`))
    (`self.GenerateRail`))
  (if (`self.StartActive`)
    (`|ExecutionSequence` :!label _label
      (:`then_0`
        (set `self.activated` true)
        (for _array_element (`SceneComponent.GetChildrenComponents` (`self.DefaultSceneRoot`) false)
          (bind _asspline_mesh_component (cast `SplineMeshComponent` _array_element))
          (set `PrimitiveComponent.bGenerateOverlapEvents` true _asspline_mesh_component)
          (add `PrimitiveComponent.OnComponentBeginOverlap` _asspline_mesh_component (delegate `OverlapRail`)))
        ;[1 1 1] Reveal Rail
        (bind _result (`BlueprintSetLibrary.Set_ToArray` (`self.Materials`)))
        (for _array_element_2 _result
          (`MaterialInstanceDynamic.SetScalarParameterValue` _array_element_2 "StartTime" (`KismetSystemLibrary.GetGameTimeInSeconds`))
          (`MaterialInstanceDynamic.SetScalarParameterValue` _array_element_2 "Speed" (`self.RailRevealSpeedModifier`)))
        (`TimelineComponent.SetPlayRate` (`self.Revealcap`) (/ (`self.RailRevealSpeedModifier`) (- (`KismetArrayLibrary.Array_Length` (`SceneComponent.GetChildrenComponents` (`self.DefaultSceneRoot`) false)) 2)))
        (`SceneComponent.SetVisibility` (`self.icing_Tube_Cap`) true false)
        (bind (_direction _time) (`Timeline|Revealcap` :!via `PlayFromStart`)
          (:`Update`
            (`SceneComponent.K2_SetWorldLocation` (`self.icing_Tube_Cap`) (`SplineComponent.GetLocationAtTime` (`self.Spline`) _time "World" true) false false)
            (`SceneComponent.K2_SetRelativeRotation` (`self.icing_Tube_Cap`) (`KismetMathLibrary.Conv_VectorToRotator` (+ (`SplineComponent.GetDirectionAtTime` (`self.Spline`) _time "Local" true) (`KismetMathLibrary.Conv_RotatorToVector` (`self.startRot`)))) false false))))
      (:`then_1`
        (bind (_direction_2 _newtrack_0) (`Timeline|Squish`)
          (:`Update`
            (`SkeletalMeshComponent.SetMorphTarget` (`self.Pouch`) "Squish" _newtrack_0 true)
            (`SceneComponent.K2_SetRelativeLocation` (`self.Collision`) (`KismetMathLibrary.MakeVector` 0.0 0.0 (+ (* _newtrack_0 -125.0) 92.964033)) false false)
            (`SceneComponent.SetVisibility` (`self.Spout`) true false)
            (`|ExecutionSequence`
              (:`then_0`
                (bind (_direction_3 _newtrack_0_2) (`Timeline|standingOn` :!via `Stop` :!label _label_2)
                  (:`Update`
                    (`SkeletalMeshComponent.SetMorphTarget` (`self.Pouch`) "Squish" _newtrack_0_2 true)
                    (`SceneComponent.K2_SetRelativeLocation` (`self.Collision`) (`KismetMathLibrary.MakeVector` 0.0 0.0 (+ (* _newtrack_0_2 -50.0) 92.964033)) false false))))
              (:`then_1`
                (bind (_direction_4 _newtrack_0_3) (`Timeline|standingOff` :!via `Stop` :!label _label_3)
                  (:`Update`
                    (`SkeletalMeshComponent.SetMorphTarget` (`self.Pouch`) "Squish" _newtrack_0_3 true)
                    (`SceneComponent.K2_SetRelativeLocation` (`self.Collision`) (`KismetMathLibrary.MakeVector` 0.0 0.0 (+ (* _newtrack_0_3 -50.0) 92.964033)) false false)))))))))
    (else
      ;[1 1 1] Start Disabled
      (bind _result_2 (`BlueprintSetLibrary.Set_ToArray` (`self.Materials`)))
      (for _array_element_3 _result_2
        (`MaterialInstanceDynamic.SetScalarParameterValue` _array_element_3 "Speed" 0.0)))))

(event `OverlapRail`
  (params (OverlappedComponent :type "PrimitiveComponent Object Reference") (OtherActor :type "Actor Object Reference") (OtherComp :type "PrimitiveComponent Object Reference") (OtherBodyIndex :type Integer) (bFromSweep :type Boolean) (SweepResult :type "HitResult Structure (by ref)"))
  ;[1 1 1] OnAttatchToRail
  (bind _asbp_player_base (cast `/Game/Blueprints/BP_PlayerBase` OtherActor))
  (`/Game/Blueprints/BP_PlayerBase.ConnectToRail` _asbp_player_base (`self.Spline`) (`self.GrindSpeed`))
  (`/Game/Blueprints/Components/Activator.ActivateAllActivatables` (`self.OnPlayerAttatch`)))

(event `/Game/Blueprints/Interfaces/IActivatable.Activate`
  (`/Engine/EditorBlueprintResources/StandardMacros.DoOnce` false :!label _label_4
    (:`Completed`
      (goto _label))))

(event `/Game/Blueprints/Interfaces/IDamageable.OnDamage`
  (params (Damage :type Integer) (Knockback :type "Vector Structure") (CanDamage :type Integer))
  (bind _returnvalue (`|BitmaskLiteral` 8))
  (if (and (== (`KismetMathLibrary.And_IntInt` CanDamage _returnvalue) _returnvalue) (not (`self.activated`)))
    (goto _label_4)))

(event `self.Trigger.OnComponentBeginOverlap`
  (params (OverlappedComponent :type "PrimitiveComponent Object Reference") (OtherActor :type "Actor Object Reference") (OtherComp :type "PrimitiveComponent Object Reference") (OtherBodyIndex :type Integer) (bFromSweep :type Boolean) (SweepResult :type "HitResult Structure (by ref)"))
  (if (and (`self.ActorHasTag` OtherActor "Player") (not (`self.activated`)))
    (goto _label_2 :!via `PlayFromStart`)))

(event `self.Trigger.OnComponentEndOverlap`
  (params (OverlappedComponent :type "PrimitiveComponent Object Reference") (OtherActor :type "Actor Object Reference") (OtherComp :type "PrimitiveComponent Object Reference") (OtherBodyIndex :type Integer))
  (if (and (`self.ActorHasTag` OtherActor "Player") (not (`self.activated`)))
    (goto _label_3 :!via `PlayFromStart`)))

(event `OnDetatch`
  (`/Game/Blueprints/Components/Activator.ActivateAllActivatables` (`self.OnPlayerDetatch`)))

(fn `GenerateRail`
  (bind (_remainder _returnvalue) (`KismetMathLibrary.FMod` (- (`SplineComponent.GetSplineLength` (`self.Spline`)) (`self.CapLength`)) (`self.MeshLength`)))
  (set `self.scaleRemainder` _remainder)
  (for _index (range _returnvalue)
    (`self.SetRailMesh` _index (+ _index 1) (`KismetMathLibrary.SafeDivide` (`self.scaleRemainder`) (`KismetMathLibrary.Conv_IntToDouble` _returnvalue)))))

(fn `SetRailCap`
  (bind _meshlength (`self.MeshLength`))
  (bind _meshlength_2 (`self.MeshLength`))
  (bind _spline (`self.Spline`))
  (bind _spline_2 (`self.Spline`))
  (bind _returnvalue (`SplineComponent.GetSplineLength` (`self.Spline`)))
  (bind _returnvalue_2 (- _returnvalue (`self.CapLength`)))
  (bind _returnvalue_3 (`AddComponent|NODE_AddSplineMeshComponent-3`))
  (bind (_min _max) (break `Box` (`StaticMesh.GetBoundingBox` (`StaticMeshComponent.StaticMesh` _returnvalue_3))))
  (set `self.CapLength` (- (.z _max) (.z _min)))
  (bind _returnvalue_4 (`KismetMaterialLibrary.CreateDynamicMaterialInstance` "/Game/Assets/Materials/IcingRail/IcingRailMaster.IcingRailMaster"))
  (`BlueprintSetLibrary.Set_Add` (`self.Materials`) _returnvalue_4)
  (`MaterialInstanceDynamic.SetScalarParameterValue` _returnvalue_4 "Offset" (* (`.ReturnValue` (`KismetMathLibrary.FMod` (- (`SplineComponent.GetSplineLength` (`self.Spline`)) (`self.CapLength`)) (`self.MeshLength`))) (`KismetMathLibrary.SafeDivide` 1.0 (`self.RailRevealSpeedModifier`))))
  (`PrimitiveComponent.SetMaterial` _returnvalue_3 0 _returnvalue_4)
  (`SceneComponent.K2_AttachToComponent` _returnvalue_3 (`self.DefaultSceneRoot`) "None" "KeepRelative" "KeepRelative" "KeepRelative" true)
  (`SplineMeshComponent.SetStartAndEnd` _returnvalue_3 (`SplineComponent.GetLocationAtDistanceAlongSpline` _spline _returnvalue_2 "Local") (`KismetMathLibrary.ClampVectorSize` (`SplineComponent.GetTangentAtDistanceAlongSpline` _spline _returnvalue_2 "Local") _meshlength_2 _meshlength_2) (`SplineComponent.GetLocationAtDistanceAlongSpline` _spline_2 _returnvalue "Local") (`KismetMathLibrary.ClampVectorSize` (`SplineComponent.GetTangentAtDistanceAlongSpline` _spline_2 _returnvalue "Local") _meshlength _meshlength) true))

(fn `SetRailMesh`
  (params (InInt :type Integer) (InInt2 :type Integer) (ScaleRemainder :type "Float (double-precision)") (Final :type Boolean))
  (bind _spline (`self.Spline`))
  (bind _spline_2 (`self.Spline`))
  (bind _returnvalue (* (+ ScaleRemainder (`self.MeshLength`)) (`KismetMathLibrary.Conv_IntToDouble` InInt2)))
  (bind _returnvalue_2 (* (+ ScaleRemainder (`self.MeshLength`)) (`KismetMathLibrary.Conv_IntToDouble` InInt)))
  (bind _returnvalue_3 (`AddComponent|NODE_AddSplineMeshComponent-0`))
  (bind (_min _max) (break `Box` (`StaticMesh.GetBoundingBox` (`StaticMeshComponent.StaticMesh` _returnvalue_3))))
  (set `self.MeshLength` (- (.y _max) (.y _min)))
  (bind _returnvalue_4 (`KismetMaterialLibrary.CreateDynamicMaterialInstance` "/Game/Assets/Materials/IcingRail/IcingRailDeform.IcingRailDeform"))
  (`BlueprintSetLibrary.Set_Add` (`self.Materials`) _returnvalue_4)
  (`MaterialInstanceDynamic.SetScalarParameterValue` _returnvalue_4 "Offset" (* InInt (`KismetMathLibrary.SafeDivide` 1.0 (`self.RailRevealSpeedModifier`))))
  (`PrimitiveComponent.SetMaterial` _returnvalue_3 0 _returnvalue_4)
  (`SceneComponent.K2_AttachToComponent` _returnvalue_3 (`self.DefaultSceneRoot`) "None" "KeepRelative" "KeepRelative" "KeepRelative" true)
  (`SplineMeshComponent.SetStartAndEnd` _returnvalue_3 (`SplineComponent.GetLocationAtDistanceAlongSpline` _spline_2 _returnvalue_2 "Local") (`KismetMathLibrary.ClampVectorSize` (`SplineComponent.GetTangentAtDistanceAlongSpline` _spline_2 _returnvalue_2 "Local") 0.0 200.0) (`SplineComponent.GetLocationAtDistanceAlongSpline` _spline _returnvalue "Local") (`KismetMathLibrary.ClampVectorSize` (`SplineComponent.GetTangentAtDistanceAlongSpline` _spline _returnvalue "Local") 0.0 200.0) true)
  (`SplineMeshComponent.SetSplineUpDir` _returnvalue_3 (`KismetMathLibrary.Vector_Up`) true))

(fn `UserConstructionScript`
  (bind _spline (`self.Spline`))
  (if (`self.GenerateRealtime`)
    (`self.GenerateRail`))
  ;[1 1 1] Icing Pouch
  (`SceneComponent.K2_SetRelativeLocationAndRotation` (`self.Pouch`) (+ (`SplineComponent.GetLocationAtTime` _spline 0.0 "Local" false) (* (`SplineComponent.GetDirectionAtTime` _spline 0.0 "Local" false) -225.0) (0.0 0.0 -40.0)) (`KismetMathLibrary.ComposeRotators` (`SplineComponent.GetRotationAtTime` (`self.Spline`) 0.0 "Local" false) (struct :`Yaw` 90.0)) false false))